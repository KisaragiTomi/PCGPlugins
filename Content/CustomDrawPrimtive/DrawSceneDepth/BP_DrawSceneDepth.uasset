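; Debug actor that captures scene world-Z height inside its Box component into a render target on BeginPlay.
; A custom tagged-box draw call fills HeightRenderTarget from the box transform and size, then a debug pass visualizes its height samples and prints the result.
; A separate Test function debug-draws voxel cavity spans within the box bounds and holds an unconnected copy of the height-draw chain.
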(event `self.ReceiveBeginPlay`
  (bind _box (`self.Box`))
  (bind _heightrendertarget (`self.HeightRenderTarget`))
  (bind _returnvalue (`SceneComponent.K2_GetComponentToWorld` _box))
  (bind _returnvalue_2 (* (`BoxComponent.GetUnscaledBoxExtent` _box) 2.0))
  (`CSDrawPrimtive.DrawTaggedBoxSceneWorldZHeight` self _returnvalue _returnvalue_2 _heightrendertarget)
  (bind _returnvalue_3 (`CSDrawPrimtive.DrawDebugBoxSceneWorldZHeightSamples` self _returnvalue _returnvalue_2 _heightrendertarget (`self.DebugPointDuration`)))
  (`KismetSystemLibrary.PrintString` (`KismetStringLibrary.Conv_IntToString` _returnvalue_3)))

(fn `Test`
  (bind (_origin _boxextent) (`KismetSystemLibrary.GetComponentBounds` (`self.Box`)))
  (`ComputeShaderBasicFunction.DebugDrawVoxelCavitySpansInBox` _origin _boxextent (struct) 64 64 5.0))

(fn `UserConstructionScript`)