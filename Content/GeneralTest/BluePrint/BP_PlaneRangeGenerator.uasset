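; Blueprint actor for plane range generation that runs Generate repeatedly on a very short looping timer, started at BeginPlay or by BPGenerate.
; GenerateTransform stores and prints the transform count from GenerateTransformsCount, which, like Generate, is defined outside these graphs.
; VisTransform debugs StoreCaptureTransforms by printing its length and drawing a temporary red arrow along each transform's forward vector.
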(event `self.ReceiveTick`
  (params (DeltaSeconds :type "Float (single-precision)")))

(event `GenerateTransform`
  (bind _returnvalue (`self.GenerateTransformsCount`))
  (`KismetSystemLibrary.PrintString` (`KismetStringLibrary.Conv_IntToString` (`KismetArrayLibrary.Array_Length` _returnvalue))))

(event `self.ReceiveBeginPlay`
  (`KismetSystemLibrary.K2_SetTimerDelegate` (delegate `CustomEvent`) 0.01 true true :!label _label))

(event `BPGenerate`
  (goto _label))

(event `CustomEvent`
  (`self.Generate`))

(event `VisTransform`
  (bind _storecapturetransforms (`self.StoreCaptureTransforms`))
  (`KismetSystemLibrary.PrintString` (`KismetStringLibrary.Conv_IntToString` (`KismetArrayLibrary.Array_Length` _storecapturetransforms)))
  (for _array_element _storecapturetransforms
    (`KismetSystemLibrary.DrawDebugArrow` (.location _array_element) (+ (.location _array_element) (* (`KismetMathLibrary.GetForwardVector` (.rotation _array_element)) 333.0)) 1.0 (struct :`R` 1.0 :`A` 1.0) 11.0 1.0)))

(fn `UserConstructionScript`)