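; Landscape Blueprint brush that alters landscape height by drawing a material into the Landmass heightmap render target.
; Initialize finds or spawns a LandmassBrushManager and passes it the landscape info.
; BrushSetup, run on construction and each RenderLayer, creates a dynamic material from position, map size, UV offset and rotation.
; RenderLayer feeds it the combined height and returns the manager's target; ClearMap clears RTResult and requests an update.
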(event `self.Initialize`
  (params (InLandscapeTransform :type "Transform Structure (by ref)") (InLandscapeSize :type "IntPoint Structure (by ref)") (InLandscapeRenderTargetSize :type "IntPoint Structure (by ref)"))
  (bind _landmasslandscapeinfo (make `LandmassLandscapeInfo` InLandscapeTransform InLandscapeSize InLandscapeRenderTargetSize))
  (bind _brushmanager (`self.BrushManager`))
  (`/Engine/EditorBlueprintResources/StandardMacros.IsValid` (`self.BrushManager`)
    (:`Is Valid`
      _)
    (:`Is Not Valid`
      (bind _outactors (`GameplayStatics.GetAllActorsOfClass` "/Landmass/Landscape/BlueprintBrushes/LandmassBrushManager.LandmassBrushManager_C"))
      (if (>= (`KismetArrayLibrary.Array_LastIndex` _outactors) 0)
        (`|VariableSetRef` _brushmanager (`|GetArrayItem` _outactors))
        (else
          (bind _returnvalue (`|SpawnActorFromClass` "/Landmass/Landscape/BlueprintBrushes/LandmassBrushManager.LandmassBrushManager_C" (`KismetMathLibrary.MakeTransform` (0.0 0.0 0.0)) "Undefined" "MultiplyWithRoot" null (struct) (struct) null))
          (`|VariableSetRef` _brushmanager _returnvalue)))))
  (if (> (`.X` (break `IntPoint` (`.LandscapeQuads` (break `LandmassLandscapeInfo` _landmasslandscapeinfo)))) 0)
    (`/Landmass/Landscape/BlueprintBrushes/LandmassBrushManager.Set Landscape Info` _brushmanager _landmasslandscapeinfo)))

(event `ClearMap`
  (bind _rt_result (`self.RT_Result`))
  (bind _returnvalue_x (`KismetMathLibrary.BreakVector` (- (`self.MapMax`) (`self.MapMin`))))
  (`KismetRenderingLibrary.ClearRenderTarget2D` _rt_result (`TextureRenderTarget2D.ClearColor` _rt_result))
  (`self.RequestLandscapeUpdate` false)
  (`KismetSystemLibrary.PrintString` (`KismetStringLibrary.Conv_DoubleToString` _returnvalue_x)))

(fn `BrushSetup`
  (bind _drawbrushmid (`self.DrawBrushMID`))
  (bind _returnvalue_x (`KismetMathLibrary.BreakVector` (- (`self.MapMax`) (`self.MapMin`))))
  (`/Landmass/Landscape/BlueprintBrushes/LandmassBrushManager.Set MPC Params` (`self.BrushManager`))
  (bind _returnvalue (`KismetMaterialLibrary.CreateDynamicMaterialInstance` (`self.UsedMaterial`)))
  (set `self.DrawBrushMID` _returnvalue)
  (`MaterialInstanceDynamic.SetVectorParameterValue` _drawbrushmid "P" (`KismetMathLibrary.Conv_VectorToLinearColor` (`self.K2_GetActorLocation`)))
  (`MaterialInstanceDynamic.SetScalarParameterValue` _drawbrushmid "Size" (/ _returnvalue_x 4.0))
  (`MaterialInstanceDynamic.SetVectorParameterValue` _drawbrushmid "UVOffset" (`KismetMathLibrary.Conv_VectorToLinearColor` (- (/ (`self.LandscapeTexUVRange`) 2.0) (0.5 0.5 0.0) (* (`self.LandscapeTexMinUV`) -0.75))))
  (`MaterialInstanceDynamic.SetScalarParameterValue` _drawbrushmid "Rotate" (`self.Rotate`)))

(fn `RenderLayer`
  (params (InParameters :type "LandscapeBrushParameters Structure (by ref)"))
  (returns (ReturnValue :type "TextureRenderTarget2D Object Reference"))
  (bind _heightmap_render_rt (`/Landmass/Landscape/BlueprintBrushes/LandmassBrushManager.Heightmap Render RT` (`self.BrushManager`)))
  (`self.BrushSetup`)
  (`MaterialInstanceDynamic.SetTextureParameterValue` (`self.DrawBrushMID`) "HeightRT" (`.CombinedResult` (break `LandscapeBrushParameters` InParameters)))
  (`KismetRenderingLibrary.ClearRenderTarget2D` _heightmap_render_rt)
  (`KismetRenderingLibrary.DrawMaterialToRenderTarget` _heightmap_render_rt (`self.DrawBrushMID`))
  (return (`/Landmass/Landscape/BlueprintBrushes/LandmassBrushManager.Heightmap Render RT` (`self.BrushManager`))))

(fn `UserConstructionScript`
  (`self.BrushSetup`))