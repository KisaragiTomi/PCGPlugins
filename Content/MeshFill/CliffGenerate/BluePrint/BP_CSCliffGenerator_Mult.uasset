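; Cliff generator Blueprint actor that fits its StaticMesh component to the size of its Box component.
; The mesh's relative scale is the scaled box extent times a constant factor, and its relative location is raised in Z by the box's half-height.
; This runs in the Construction Script, at BeginPlay and again every Tick, after the parent class's logic.
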(event `self.ReceiveBeginPlay`
  (bind _staticmesh (`self.StaticMesh`))
  (bind _returnvalue (`BoxComponent.GetScaledBoxExtent` (`self.Box`)))
  (bind (_returnvalue_x _returnvalue_y _returnvalue_z) (`KismetMathLibrary.BreakVector` (/ _returnvalue 1.0)))
  (`parent.ReceiveBeginPlay`)
  (`SceneComponent.SetRelativeScale3D` _staticmesh (* _returnvalue 0.0205) :!label _label)
  (`SceneComponent.K2_SetRelativeLocation` _staticmesh (`KismetMathLibrary.MakeVector` 0.0 0.0 _returnvalue_z) false false))

(event `self.ReceiveTick`
  (params (DeltaSeconds :type "Float (single-precision)"))
  (`parent.ReceiveTick` DeltaSeconds)
  (goto _label))

(fn `UserConstructionScript`
  (bind _staticmesh (`self.StaticMesh`))
  (bind _returnvalue (`BoxComponent.GetScaledBoxExtent` (`self.Box`)))
  (bind (_returnvalue_x _returnvalue_y _returnvalue_z) (`KismetMathLibrary.BreakVector` (/ _returnvalue 1.0)))
  (`parent.UserConstructionScript`)
  (`SceneComponent.SetRelativeScale3D` _staticmesh (* _returnvalue 0.0205))
  (`SceneComponent.K2_SetRelativeLocation` _staticmesh (`KismetMathLibrary.MakeVector` 0.0 0.0 _returnvalue_z) false false))