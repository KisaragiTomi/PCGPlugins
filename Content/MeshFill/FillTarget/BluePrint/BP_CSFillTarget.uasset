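; Mesh-fill target actor that exposes events to run a fill pass, a curvature post test and a debug render-target copy.
; Construction resets the box's relative rotation and zeroes actor pitch.
; It also gives the light and post-mask captures dynamic post-process materials for scene-light threshold and world-noise max height.
; The fill and curvature work happens in functions defined outside this graph.
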(event `CopyTexture`
  (`ComputeShaderBasicFunction.CopyTexture` (`self.RT_DebugView`) "/TAToolsPlugin/MeshFill/FillTarget/Material/RT_UVTest.RT_UVTest")
  (`KismetSystemLibrary.PrintString` (`KismetStringLibrary.Conv_RotatorToString` (`SceneComponent.RelativeRotation` (`self.Box`)))))

(event `BP_FillTarget`
  (`self.FillTarget` 5))

(event `BP_CurvaturePostTest`
  (`self.CurvaturePostTest`))

(fn `UserConstructionScript`
  (bind (_returnvalue_roll _returnvalue_pitch _returnvalue_yaw) (`KismetMathLibrary.BreakRotator` (`self.K2_GetActorRotation`)))
  (`SceneComponent.K2_SetRelativeRotation` :`self` (`self.Box`))
  (`self.K2_SetActorRotation` (`KismetMathLibrary.MakeRotator` _returnvalue_roll 0.0 _returnvalue_yaw))
  (`|ExecutionSequence`
    (:`then_0`
      (bind _returnvalue (`KismetMaterialLibrary.CreateDynamicMaterialInstance` "/TAToolsPlugin/MeshFill/FillTarget/Material/MI_PP_SceneLight.MI_PP_SceneLight"))
      (`MaterialInstanceDynamic.SetScalarParameterValue` _returnvalue "Threashould" (`self.SceneLightThreashould`))
      (set `SceneCaptureComponent2D.PostProcessSettings` (make `PostProcessSettings` :`WeightedBlendables` (make `WeightedBlendables` (`|MakeArray` (make `WeightedBlendable` 1.0 _returnvalue) :!type "WeightedBlendable Structure"))) (`self.CaptureLight`)))
    (:`then_1`
      (bind _returnvalue_2 (`KismetMaterialLibrary.CreateDynamicMaterialInstance` "/TAToolsPlugin/MeshFill/FillTarget/Material/MI_PP_SceneWorldNoise.MI_PP_SceneWorldNoise"))
      (`MaterialInstanceDynamic.SetScalarParameterValue` _returnvalue_2 "HeightMax" (`self.SceneWorldNoiseHeightMax`))
      (set `SceneCaptureComponent2D.PostProcessSettings` (make `PostProcessSettings` :`WeightedBlendables` (make `WeightedBlendables` (`|MakeArray` (make `WeightedBlendable` 1.0 _returnvalue_2) :!type "WeightedBlendable Structure"))) (`self.CapturePostMask`)))))