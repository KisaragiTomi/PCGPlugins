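; Actor wrapper around a FluxModifierSource component that feeds flux modifiers into the shallow water simulation.
; Construction builds the source, passing the restart-simulation-on-edit flag, and snaps a box component onto it.
; AddModifiers forwards modifiers to the source.
; On BeginPlay, if destroy-on-finish is set and the duration is non-negative, the actor's lifespan is set to just past that duration.
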(event `self.ReceiveBeginPlay`
  (bind _duration (`/TAToolsPlugin/ShallowWater/Material30/Simulation/Modifiers/Components/BP_FluxModifierComponent.Duration` (`self.FluxModifierSource`)))
  (if (`self.DestroyonOnFinish`)
    (if (>= _duration 0.0)
      (`self.SetLifeSpan` (+ _duration 0.02)))))

(fn `AddModifiers`
  (params (Modifiers :type "Array of /TAToolsPlugin/ShallowWater/Material30/Simulation/Modifiers/Components/BP_FluxModifierComponent Object Reference (by ref)"))
  (returns (Remove :type Boolean))
  (bind _finalized (`/TAToolsPlugin/ShallowWater/Material30/Simulation/Modifiers/Components/BP_FluxModifierComponent.AddModifier` (`self.FluxModifierSource`) Modifiers))
  (return _finalized))

(fn `UserConstructionScript`
  (`/TAToolsPlugin/ShallowWater/Material30/Simulation/Modifiers/Components/BP_FluxModifierComponent.ConstructComponent` (`self.FluxModifierSource`) (`self.RestartSimulationOnEdit`))
  (bind _returnvalue (`AddComponent|NODE_AddBoxComponent-0` :`bManualAttachment` true))
  (`SceneComponent.K2_AttachToComponent` _returnvalue (`self.FluxModifierSource`) "None" "SnapToTarget" "SnapToTarget" "SnapToTarget" true))