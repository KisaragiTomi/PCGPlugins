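; Data asset preset that defines the optical look of a shallow water surface: scattering, absorption, clarity, phase, behind and overlay colors.
; ApplyMaterial forwards to SetSurfaceColor, which writes these values to material instance parameters whose names end in a given postfix.
; Clarity scales the alpha of absorption directly and that of scattering inversely, so one value drives both in opposite directions.
; CopyProperties copies all preset values to a destination preset.
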(fn `ApplyMaterial`
  (params (MaterialInstances :type "Array of MaterialInstanceDynamic Object Reference") (Postfix :type String))
  (`self.SetSurfaceColor` MaterialInstances Postfix))

(fn `CopyProperties`
  (params (Destination :type "/Game/ShallowWater/Material30/Surface/Blueprints/PDA_FluxSurfacePreset Object Reference"))
  (set `/Game/ShallowWater/Material30/Surface/Blueprints/PDA_FluxSurfacePreset.Clarity` (`self.Clarity`) (`local.Destination`))
  (set `/Game/ShallowWater/Material30/Surface/Blueprints/PDA_FluxSurfacePreset.Scattering` (`self.Scattering`) (`local.Destination`))
  (set `/Game/ShallowWater/Material30/Surface/Blueprints/PDA_FluxSurfacePreset.Absorption` (`self.Absorption`) (`local.Destination`))
  (set `/Game/ShallowWater/Material30/Surface/Blueprints/PDA_FluxSurfacePreset.Overlay` (`self.Overlay`) (`local.Destination`))
  (set `/Game/ShallowWater/Material30/Surface/Blueprints/PDA_FluxSurfacePreset.Behind` (`self.Behind`) (`local.Destination`))
  (set `/Game/ShallowWater/Material30/Surface/Blueprints/PDA_FluxSurfacePreset.PhaseG` (`self.PhaseG`) (`local.Destination`)))

(fn `SetSurfaceColor`
  (params (Materials :type "Array of MaterialInstanceDynamic Object Reference (by ref)") (Postfix :type String))
  (bind _clarity (`self.Clarity`))
  (`MaterialInstanceDynamic.SetVectorParameterValue` (`local.Materials`) (`KismetStringLibrary.Conv_StringToName` (`KismetStringLibrary.Concat_StrStr` "SurfaceScattering" Postfix)) (* (`self.Scattering`) (make `LinearColor` 1.0 1.0 1.0 (/ 1.0 _clarity))))
  (`MaterialInstanceDynamic.SetVectorParameterValue` (`local.Materials`) (`KismetStringLibrary.Conv_StringToName` (`KismetStringLibrary.Concat_StrStr` "SurfaceAbsorption" Postfix)) (* (`self.Absorption`) (make `LinearColor` 1.0 1.0 1.0 _clarity)))
  (`MaterialInstanceDynamic.SetScalarParameterValue` (`local.Materials`) (`KismetStringLibrary.Conv_StringToName` (`KismetStringLibrary.Concat_StrStr` "SurfacePhaseG" Postfix)) (`self.PhaseG`))
  (`MaterialInstanceDynamic.SetVectorParameterValue` (`local.Materials`) (`KismetStringLibrary.Conv_StringToName` (`KismetStringLibrary.Concat_StrStr` "ColorBehind" Postfix)) (`self.Behind`))
  (`MaterialInstanceDynamic.SetVectorParameterValue` (`local.Materials`) (`KismetStringLibrary.Conv_StringToName` (`KismetStringLibrary.Concat_StrStr` "SurfaceOverlay" Postfix)) (`self.Overlay`)))