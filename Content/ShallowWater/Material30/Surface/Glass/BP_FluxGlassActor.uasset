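; Glass actor for Flux water surfaces, with an empty ConstructMeshes hook.
; On construction and BeginPlay it creates absorption, scattering and inside material instances and has a BPI_FluxSurface actor apply surface data to them.
; It notifies SDF volumes of shape changes if it is an SDF source.
; Per-tag mesh setup for volume, outside, inside and phantom layers exists but is unwired in ApplyGlassSettingsByTag.
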(event `self.ReceiveBeginPlay`
  (`self.CreateMaterials`)
  (bind _surfaceabstract (`self.GetWorldSurface`))
  (`self.ApplySurfaceData` _surfaceabstract)
  (`self.ApplyGlassSettingsByTag`)
  (`self.GenerateDistanceFields`))

(event `/TAToolsPlugin/ShallowWater/Material30/Surface/Blueprints/BPI_FluxSurfaceMeshActor.ApplySurfaceData`
  (params (SurfaceActor :type "Actor Object Reference"))
  ;[1 0.209 0.03491] Event executed by surface actor to apply surface data on this mesh and material.
  (`/Engine/EditorBlueprintResources/StandardMacros.IsValid` SurfaceActor
    (:`Is Valid`
      (message `/TAToolsPlugin/ShallowWater/Material30/Surface/Blueprints/BPI_FluxSurface.ApplySurfaceMaterialData` SurfaceActor (`self.SurfaceInstances`) true true))))

(fn `ApplyGlassSettingsByTag`
  (`|ExecutionSequence`))

(fn `ConstructMeshes`
  (locals (SplineIndex :type Integer)))

(fn `CreateMaterials`
  (`|ExecutionSequence`
    (:`then_0`
      (`KismetArrayLibrary.Array_Clear` (`self.SurfaceInstances`)))
    (:`then_1`
      (`self.AbsorptionInstance`
        (:`then`)
        (:`else`
          (bind _returnvalue (`KismetMaterialLibrary.CreateDynamicMaterialInstance` (`self.AbsorptionMaterial`)))
          (set `self.AbsorptionInstance` _returnvalue))))
    (:`then_2`
      (`self.ScatteringInstance`
        (:`then`)
        (:`else`
          (bind _returnvalue_2 (`KismetMaterialLibrary.CreateDynamicMaterialInstance` (`self.ScatteringMaterial`)))
          (set `self.ScatteringInstance` _returnvalue_2))))
    (:`then_3`
      (`self.GlassInsideMaterial`
        (:`then`
          (bind _returnvalue_3 (`KismetMaterialLibrary.CreateDynamicMaterialInstance` (`self.GlassInsideMaterial`)))
          (set `self.InsideInstance` _returnvalue_3))
        (:`else`)))
    (:`then_4`
      (bind _output_get (set `self.SurfaceInstances` (`|MakeArray` (`self.AbsorptionInstance`) (`self.ScatteringInstance`) (`self.InsideInstance`))))
      (`KismetArrayLibrary.Array_RemoveItem` _output_get))))

(fn `GenerateDistanceFields`
  (if (`KismetSystemLibrary.DoesImplementInterface` self "/TAToolsPlugin/ShallowWater/Material30/Tools/DistanceField/Blueprints/BPI_SDFSource.BPI_SDFSource_C")
    (bind _outactors (`GameplayStatics.GetAllActorsWithInterface` "/TAToolsPlugin/ShallowWater/Material30/Tools/DistanceField/Blueprints/BPI_SDFVolume.BPI_SDFVolume_C"))
    (message `/TAToolsPlugin/ShallowWater/Material30/Tools/DistanceField/Blueprints/BPI_SDFVolume.OnCapturedShapeChanged` _outactors self)))

(fn `GetWorldSurface`
  (returns (SurfaceAbstract :type "Actor Object Reference"))
  (if (`KismetSystemLibrary.DoesImplementInterface` (`self.GetOwner`) "/TAToolsPlugin/ShallowWater/Material30/Surface/Blueprints/BPI_FluxSurface.BPI_FluxSurface_C")
    (return (`self.GetOwner`))
    (else
      (bind _outactors (`GameplayStatics.GetAllActorsWithInterface` "/TAToolsPlugin/ShallowWater/Material30/Surface/Blueprints/BPI_FluxSurface.BPI_FluxSurface_C"))
      (if (> (`KismetArrayLibrary.Array_Length` _outactors) 0)
        (return (`|GetArrayItem` _outactors))))))

(fn `GlassMeshSettings`
  (params (Mesh :type "MeshComponent Object Reference") (SortPriority :type Integer) (BaseMaterial :type "MaterialInterface Object Reference") (OverlayMaterial :type "MaterialInterface Object Reference") (EnableCollision :type Boolean) (ReverseCulling :type Boolean) (CastShadow :type Boolean))
  (`|ExecutionSequence`
    (:`then_0`
      (`PrimitiveComponent.SetTranslucentSortPriority` (`local.Mesh`) (`local.SortPriority`))
      (`PrimitiveComponent.SetMaterial` (`local.Mesh`) 0 (`local.BaseMaterial`))
      (`MeshComponent.SetOverlayMaterial` (`local.Mesh`) (`local.OverlayMaterial`)))
    (:`then_1`
      (if (`local.EnableCollision`)
        (`PrimitiveComponent.SetCollisionEnabled` (`local.Mesh`) "QueryAndPhysics")
        (`PrimitiveComponent.SetCollisionObjectType` (`local.Mesh`) "ECC_WorldStatic")
        (`PrimitiveComponent.SetCollisionResponseToChannel` (`local.Mesh`) "ECC_Camera" "ECR_Block")
        (else
          (`PrimitiveComponent.SetCollisionEnabled` (`local.Mesh`) "NoCollision"))))
    (:`then_2`
      (bind _asstatic_mesh_component (cast `StaticMeshComponent` (`local.Mesh`)))
      (`StaticMeshComponent.SetReverseCulling` _asstatic_mesh_component (`local.ReverseCulling`))
      (`PrimitiveComponent.SetCastShadow` _asstatic_mesh_component (`local.CastShadow`)))))

(fn `RefreshSurfaceData`
  (`self.Surface Actor`
    (:`then`
      (if (`KismetSystemLibrary.DoesImplementInterface` (`self.Surface Actor`) "/TAToolsPlugin/ShallowWater/Material30/Surface/Blueprints/BPI_FluxSurface.BPI_FluxSurface_C")
        (`self.ApplySurfaceData` (`self.Surface Actor`))
        (else
          (set `self.Surface Actor` null))))
    (:`else`
      (bind _outactors (`GameplayStatics.GetAllActorsWithInterface` "/TAToolsPlugin/ShallowWater/Material30/Surface/Blueprints/BPI_FluxSurface.BPI_FluxSurface_C"))
      (for _array_element _outactors
        (`self.ApplySurfaceData` _array_element)))))

(fn `UserConstructionScript`
  (locals (TempMesh :type "SplineMeshComponent Object Reference"))
  (`self.CreateMaterials`)
  (bind _surfaceabstract (`self.GetWorldSurface`))
  (`self.ApplySurfaceData` _surfaceabstract)
  (`self.ConstructMeshes`)
  (`self.ApplyGlassSettingsByTag`)
  (`self.GenerateDistanceFields`))