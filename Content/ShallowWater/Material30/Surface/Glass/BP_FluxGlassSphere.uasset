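; BP_FluxGlassSphere is a glass sphere Blueprint in the ShallowWater Flux surface content that describes itself as a signed distance field shape source.
; GetShapes returns one SDF shape from the actor's location and rotation, with scale multiplied by SphereRadius and radius taken from that scale's X axis.
; GetSourceType reports a fixed enum type, and both BeginPlay and the construction script add no logic of their own.
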(fn `GetShapes`
  (returns (Shapes :type "Array of /TAToolsPlugin/ShallowWater/Material30/Tools/DistanceField/Blueprints/BS_SDFShape Structure"))
  (bind _returnvalue (* (`self.GetActorScale3D`) (`self.SphereRadius`)))
  (return (`|MakeArray` (make `/TAToolsPlugin/ShallowWater/Material30/Tools/DistanceField/Blueprints/BS_SDFShape` (`KismetMathLibrary.MakeTransform` (`self.K2_GetActorLocation`) (`self.K2_GetActorRotation`) _returnvalue) (+ (.x _returnvalue) 0.0)))))

(fn `GetSourceType`
  (returns (Type :type "/TAToolsPlugin/ShallowWater/Material30/Tools/DistanceField/Blueprints/BPE_SDFSourceType Enum"))
  (return "NewEnumerator0"))

(fn `UserConstructionScript`
  (`parent.UserConstructionScript`))