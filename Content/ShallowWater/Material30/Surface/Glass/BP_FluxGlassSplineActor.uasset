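; Spline-based glass actor for the Flux shallow water system, extending a parent that handles shared material setup.
; Builds tagged spline meshes per segment for the absorption volume, outer and inner glass, frame and simulation phantoms.
; An extra cross-section plane uses a dynamic material fed by SDF volume data to render the SDF in top-down scene capture.
; PrepareMaterial refreshes that SDF from the linked cross-section actor when valid.
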(event `/TAToolsPlugin/ShallowWater/Material30/Tools/DistanceField/Blueprints/BPI_SDFSource.PrepareMaterial`
  (params (Material :type "MaterialInstanceDynamic Object Reference"))
  ;[0.3281 0.4341 1] Settings applied when SDF volume is updated
  (bind _output_get (set `self.MeshCrossectionSDF` (select `bool` (`KismetSystemLibrary.IsValid` (`self.MeshCrossectionActor`)) :`false` (`self.MeshCrossectionSDF`) :`true` (`/TAToolsPlugin/ShallowWater/Material30/Tools/DistanceField/Blueprints/BP_SDFCrossection.VolumeDataAsset` (`self.MeshCrossectionActor`)))))
  (`/TAToolsPlugin/ShallowWater/Material30/Tools/DistanceField/Blueprints/PDA_FluxSignedDistanceField.ApplyMaterialParameters` _output_get (`|MakeArray` (`self.CrossectionInstance`)) "" false))

(fn `ConstructMeshes`
  (locals (SplineIndex :type Integer))
  (`self.SplineGlassMesh`
    (:`then`
      (for _index (range (+ (- (`SplineComponent.GetNumberOfSplinePoints` (`self.Spline`)) 2) 1))
        (set `local.SplineIndex` _index)
        (`|ExecutionSequence`
          (:`then_0`
            ;[0.6582 1 0.7465] Base: Absorption, Overlay: Scattering + Waterline
            (`self.AbsorptionInstance`
              (:`then`
                (`self.CreateSplineMesh` (`local.SplineIndex`) (`self.SplineGlassMesh`) "GlassVolume" (`self.Spline`)))
              (:`else`)))
          (:`then_1`
            ;[1 0.2948 0.2948] Glass outside
            (`self.GlassOutsideMaterial`
              (:`then`
                (`self.CreateSplineMesh` (`local.SplineIndex`) (`self.SplineGlassMesh`) "GlassOutside" (`self.Spline`)))
              (:`else`)))
          (:`then_2`
            ;[1 0.4733 0.3471] Glass inside
            (`self.GlassInsideMaterial`
              (:`then`
                (`self.CreateSplineMesh` (`local.SplineIndex`) (`self.SplineGlassMesh`) "GlassInside" (`self.Spline`)))
              (:`else`)))
          (:`then_3`
            ;[1 0.6838 0.4214] Frame mesh
            (bind _splineglassframe (`self.SplineGlassFrame`)
              (:`then`
                (`self.CreateSplineMesh` (`local.SplineIndex`) _splineglassframe "GlassFrame" (`self.Spline`)))
              (:`else`)))
          (:`then_4`
            ;[0.1704 0.2706 1] Fluid ground phantom
            (`self.SimulationPhantomMaterial`
              (:`then`
                (`|ExecutionSequence`
                  (:`then_0`
                    (`self.CreateSplineMesh` (`local.SplineIndex`) (`self.SplineGlassMesh`) "GlassPhantom" (`self.Spline`)))
                  (:`then_1`
                    (bind _splineglassframe_2 (`self.SplineGlassFrame`)
                      (:`then`
                        (`self.CreateSplineMesh` (`local.SplineIndex`) _splineglassframe_2 "GlassPhantom" (`self.Spline`)))
                      (:`else`)))))
              (:`else`)))
          (:`then_5`
            ;[0.3135 0.1663 0.2582] Crossection (special plane mesh used for rendering SDF in top down scene capture view)
            (`self.CrossectionInstance`
              (:`then`
                (bind _returnvalue (`self.CreateSplineMesh` (`local.SplineIndex`) (`self.SplineGlassCrossection`) "GlassCrossection" (`self.Spline`)))
                (`PrimitiveComponent.SetMaterial` _returnvalue 0 (`self.CrossectionInstance`)))
              (:`else`))))))
    (:`else`)))

(fn `CreateMaterials`
  (`parent.CreateMaterials`)
  (`self.InitializeCrossection`))

(fn `CreateSplineMesh`
  (params (SplineIndex :type Integer) (NewMesh :type "StaticMesh Object Reference") (Tag :type "Name (by ref)") (Spline :type "SplineComponent Object Reference"))
  (returns (ReturnValue :type "MeshComponent Object Reference"))
  (locals (TempMesh :type "SplineMeshComponent Object Reference"))
  (bind _splineindex (`local.SplineIndex`))
  (bind _spline (`local.Spline`))
  (bind _spline_2 (`local.Spline`))
  (bind _returnvalue (+ (`local.SplineIndex`) 1))
  (bind _returnvalue_2 (`AddComponent|NODE_AddSplineMeshComponent-3`))
  (bind _output_get (set `local.TempMesh` _returnvalue_2))
  (`KismetArrayLibrary.Array_Add` (`ActorComponent.ComponentTags` _output_get) (`local.Tag`))
  (`SplineMeshComponent.SetStartAndEnd` (`local.TempMesh`) (`SplineComponent.GetLocationAtSplinePoint` _spline _splineindex "Local") (`SplineComponent.GetTangentAtSplinePoint` _spline _splineindex "Local") (`SplineComponent.GetLocationAtSplinePoint` _spline_2 _returnvalue "Local") (`SplineComponent.GetTangentAtSplinePoint` _spline_2 _returnvalue "Local") false)
  (`SplineMeshComponent.SetForwardAxis` (`local.TempMesh`) "X" true)
  (`StaticMeshComponent.SetStaticMesh` (`local.TempMesh`) (`local.NewMesh`))
  (`SceneComponent.K2_AttachToComponent` (`local.TempMesh`) (`local.Spline`) "None" "KeepRelative" "KeepRelative" "KeepRelative" true)
  (return (`local.TempMesh`)))

(fn `GetShapes`
  (returns (Shapes :type "Array of /TAToolsPlugin/ShallowWater/Material30/Tools/DistanceField/Blueprints/BS_SDFShape Structure"))
  (return))

(fn `GetSourceType`
  (returns (Type :type "/TAToolsPlugin/ShallowWater/Material30/Tools/DistanceField/Blueprints/BPE_SDFSourceType Enum"))
  (return "NewEnumerator1"))

(fn `InitializeCrossection`
  (`self.CrossectionInstance`
    (:`then`
      _)
    (:`else`
      (bind _meshcrossectionmaterial (`self.MeshCrossectionMaterial`)
        (:`then`
          (bind _returnvalue (`KismetMaterialLibrary.CreateDynamicMaterialInstance` _meshcrossectionmaterial))
          (set `self.CrossectionInstance` _returnvalue))
        (:`else`))))
  (bind _meshcrossectionsdf (`self.MeshCrossectionSDF`)
    (:`then`
      (`/TAToolsPlugin/ShallowWater/Material30/Tools/DistanceField/Blueprints/PDA_FluxSignedDistanceField.ApplyMaterialParameters` _meshcrossectionsdf (`|MakeArray` (`self.CrossectionInstance`)) "" false))
    (:`else`)))

(fn `UserConstructionScript`
  (locals (TempMesh :type "SplineMeshComponent Object Reference") (SplineIndex :type Integer))
  (`parent.UserConstructionScript`))