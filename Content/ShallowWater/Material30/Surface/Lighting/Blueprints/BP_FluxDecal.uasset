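; BP_FluxDecal is a mesh-based decal actor for the shallow water surface system that receives surface data from a surface actor.
; The construction script scales DecalMesh from Size.
; CreateMaterials makes a dynamic material instance once and sets the translucency sort priority.
; ApplySurfaceData passes that instance back to the surface actor through ApplySurfaceMaterialDataMessage, requesting domain and color data.
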(event `/TAToolsPlugin/ShallowWater/Material30/Surface/Blueprints/BPI_FluxSurfaceMeshActor.ApplySurfaceData`
  (params (SurfaceActor :type "Actor Object Reference"))
  (bind _materialinstance (`self.MaterialInstance`)
    (:`then`
      (message `/TAToolsPlugin/ShallowWater/Material30/Surface/Blueprints/BPI_FluxSurface.ApplySurfaceMaterialData` SurfaceActor (`|MakeArray` _materialinstance) true true))
    (:`else`)))

(fn `CreateMaterials`
  (`self.MaterialInstance`
    (:`then`)
    (:`else`
      (bind _returnvalue (`PrimitiveComponent.CreateDynamicMaterialInstance` (`self.DecalMesh`) 0 (`self.Material`) "None"))
      (set `self.MaterialInstance` _returnvalue)
      (`PrimitiveComponent.SetTranslucentSortPriority` (`self.DecalMesh`) (`self.TranslucencySortPriority`)))))

(fn `UserConstructionScript`
  (`parent.UserConstructionScript`)
  (`SceneComponent.SetWorldScale3D` (`self.DecalMesh`) (* (`self.Size`) 0.01)))