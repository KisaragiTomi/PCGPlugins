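; BP_FluxPointLight is a point-light actor for the ShallowWater surface lighting, pairing a shape mesh with an optional PointLight component.
; ApplyParameters extends its parent, scales the mesh to match Radius, then either sets the light's shadows, underwater color and attenuation radius or destroys the component when AddLightComponent is off.
; SetRadius stores a new radius and reapplies the parameters.
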(fn `ApplyParameters`
  (`parent.ApplyParameters`)
  (`|ExecutionSequence`
    (:`then_0`
      (`SceneComponent.K2_SetRelativeTransform` (`self.ShapeMesh`) (`KismetMathLibrary.MakeTransform` (0.0 0.0 0.0) (struct) (`KismetMathLibrary.Conv_DoubleToVector` (/ (`self.Radius`) 50.0))) false false))
    (:`then_1`
      (if (`self.AddLightComponent`)
        (`LightComponentBase.SetCastShadows` (`self.PointLight`) (`self.CastShadows`))
        (`LightComponent.SetLightColor` (`self.PointLight`) (`self.LightColorUnderWater`) true)
        (`LocalLightComponent.SetAttenuationRadius` (`self.PointLight`) (`self.Radius`))
        (else
          (`self.PointLight`
            (:`then`
              (`ActorComponent.K2_DestroyComponent` (`self.PointLight`)))
            (:`else`)))))))

(fn `SetRadius`
  (params (Radius :type "Float (double-precision)"))
  (set `self.Radius` Radius)
  (`self.ApplyParameters`))

(fn `UserConstructionScript`
  (`parent.UserConstructionScript`))