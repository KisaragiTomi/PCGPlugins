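; BP_FluxSpotLight is a spot light Blueprint for the ShallowWater surface lighting, extending a parent through an ApplyParameters override.
; After the parent call, it sets intensity, cone angles and radius on the SpotLight, deriving the inner cone from the outer.
; It scales and offsets ShapeMesh along X to match the cone, using the angle's tangent for width.
; AddLightComponent either applies the shadow setting or destroys the SpotLight.
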(fn `ApplyParameters`
  (bind _returnvalue (/ (`self.ConeRadius`) 100.0))
  (bind _returnvalue_2 (* _returnvalue (* (`KismetMathLibrary.DegTan` (`self.ConeAngle`)) 2.0)))
  (`parent.ApplyParameters`)
  (`|ExecutionSequence`
    (:`then_0`
      (`LightComponent.SetIntensity` (`self.SpotLight`) (`self.LightIntensity`))
      (`SpotLightComponent.SetOuterConeAngle` (`self.SpotLight`) (`self.ConeAngle`))
      (`SpotLightComponent.SetInnerConeAngle` (`self.SpotLight`) (* (`self.ConeAngle`) 0.75))
      (`LocalLightComponent.SetAttenuationRadius` (`self.SpotLight`) (`self.ConeRadius`)))
    (:`then_1`
      (`SceneComponent.K2_SetRelativeTransform` (`self.ShapeMesh`) (`KismetMathLibrary.MakeTransform` (`KismetMathLibrary.MakeVector` (* 50.0 _returnvalue)) (struct) (`KismetMathLibrary.MakeVector` _returnvalue _returnvalue_2 _returnvalue_2)) false false))
    (:`then_2`
      (if (`self.AddLightComponent`)
        (`LightComponentBase.SetCastShadows` (`self.SpotLight`) (`self.CastShadows`))
        (else
          (`self.SpotLight`
            (:`then`
              (`ActorComponent.K2_DestroyComponent` (`self.SpotLight`)))
            (:`else`)))))))

(fn `UserConstructionScript`
  (`parent.UserConstructionScript`))