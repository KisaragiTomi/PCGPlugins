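; Jump flood component that generates a distance field from a source texture into the Result render target, as a shallow-water tool.
; Generate seeds one of two ping-pong render targets (RG16f, or RG32f for high precision) through the source material.
; The iteration material then runs passes with power-of-two step lengths, halving from a size-derived maximum down to one.
; The result material converts the final seeds into the SDF, scaled by Normalization.
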(fn `Generate`
  (params (SourceTexture :type "TextureRenderTarget2D Object Reference (by ref)") (Normalization :type "Float (double-precision)" :default 1.0) (HighPrecission :type Boolean) (Iterations :type Byte :default 16) (Offset :type "Float (double-precision)"))
  (locals (Flip :type Integer) (StepCount :type Integer) (CurrentTexture :type "TextureRenderTarget2D Object Reference"))
  (bind _sourcetexture (`local.SourceTexture`))
  (`|ExecutionSequence`
    (:`then_0`
      ;[1 0.4323 0.4323] Init
      (set `self.Size X` (`TextureRenderTarget2D.SizeX` _sourcetexture))
      (set `self.Size Y` (`TextureRenderTarget2D.SizeY` _sourcetexture))
      (set `local.StepCount` (- (`KismetMathLibrary.FFloor` (`KismetMathLibrary.Log` (`KismetMathLibrary.Conv_IntToDouble` (`KismetMathLibrary.Max` (`self.Size X`) (`self.Size Y`))) 2.0)) 1)))
    (:`then_1`
      (`KismetArrayLibrary.Array_Clear` (`self.TempTextures`))
      (for _ (range 2)
        (bind _returnvalue (`KismetRenderingLibrary.CreateRenderTarget2D` (`self.Size X`) (`self.Size Y`) (select `bool` (`local.HighPrecission`) :`false` "RTF_RG16f" :`true` "RTF_RG32f" :!type "ETextureRenderTargetFormat Enum")))
        (`KismetArrayLibrary.Array_Add` (`self.TempTextures`) _returnvalue))
      (set `local.Flip` 0)
      (set `local.CurrentTexture` (`|GetArrayItem` (`self.TempTextures`) (`local.Flip`))))
    (:`then_2`
      ;[0.8432 1 0.7183] Rendering source instance
      (`self.SourceInstance`
        (:`then`
          _)
        (:`else`
          (bind _returnvalue_2 (`KismetMaterialLibrary.CreateDynamicMaterialInstance` (`self.SourceMaterial`)))
          (set `self.SourceInstance` _returnvalue_2)))
      (`MaterialInstanceDynamic.SetTextureParameterValue` (`self.SourceInstance`) "Surce" (`local.SourceTexture`))
      (`MaterialInstanceDynamic.SetScalarParameterValue` (`self.SourceInstance`) "Iterations" (`KismetMathLibrary.Conv_ByteToDouble` (`local.Iterations`)))
      (`MaterialInstanceDynamic.SetScalarParameterValue` (`self.SourceInstance`) "Offset" (`local.Offset`))
      (`KismetRenderingLibrary.DrawMaterialToRenderTarget` (`local.CurrentTexture`) (`self.SourceInstance`)))
    (:`then_3`
      ;[1 0.6551 0.1922] Render iterations
      (`self.IterationInstance`
        (:`then`
          _)
        (:`else`
          (bind _returnvalue_3 (`KismetMaterialLibrary.CreateDynamicMaterialInstance` (`self.IterationMaterial`)))
          (set `self.IterationInstance` _returnvalue_3)))
      (for _index (range (+ (`local.StepCount`) 1))
        (`MaterialInstanceDynamic.SetScalarParameterValue` (`self.IterationInstance`) "StepLength" (`KismetMathLibrary.MultiplyMultiply_FloatFloat` 2.0 (`KismetMathLibrary.Conv_IntToDouble` (- (`local.StepCount`) _index))))
        (`MaterialInstanceDynamic.SetTextureParameterValue` (`self.IterationInstance`) "SeedTexture" (`local.CurrentTexture`))
        (set `local.Flip` (- 1 (`local.Flip`)))
        (set `local.CurrentTexture` (`|GetArrayItem` (`self.TempTextures`) (`local.Flip`)))
        (`KismetRenderingLibrary.DrawMaterialToRenderTarget` (`local.CurrentTexture`) (`self.IterationInstance`))))
    (:`then_4`
      ;[0.9573 0.7688 1] Render final SDF
      (`self.ResultInstance`
        (:`then`
          _)
        (:`else`
          (bind _returnvalue_4 (`KismetMaterialLibrary.CreateDynamicMaterialInstance` (`self.ResultMaterial`)))
          (set `self.ResultInstance` _returnvalue_4)))
      (`MaterialInstanceDynamic.SetTextureParameterValue` (`self.ResultInstance`) "SeedTexture" (`local.CurrentTexture`))
      (`MaterialInstanceDynamic.SetScalarParameterValue` (`self.ResultInstance`) "Scale" (`local.Normalization`))
      (`KismetRenderingLibrary.DrawMaterialToRenderTarget` (`self.Result`) (`self.ResultInstance`)))))