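; Tool actor that bakes a 2D signed distance field from a static mesh's cross-section on construction and BeginPlay.
; An orthographic scene capture renders the mesh with a cross-section material into a power-of-two render target, framed by padded, square YZ bounds.
; An optional jump flood pass generates the distance field in that same target.
; A PDA_FluxSignedDistanceField stores texture, placement and range, and feeds the debug preview material.
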(event `self.ReceiveBeginPlay`
  (`self.InitializeAll`)
  (`self.Repaint`))

(fn `InitializeAll`
  (`self.InitializeMesh`)
  (`self.InitializeRenderTargets`)
  (`self.InitializeSceneCapture`)
  (`self.InitializeDataAsset`)
  (`self.InitializeDebug`))

(fn `InitializeDataAsset`
  (bind (_relativelocation_x _relativelocation_y _relativelocation_z) (`KismetMathLibrary.BreakVector` (`SceneComponent.RelativeLocation` (`self.SceneCaptureComponent2D`))))
  (bind (_relativescale3d_x _relativescale3d_y _relativescale3d_z) (`KismetMathLibrary.BreakVector` (`SceneComponent.RelativeScale3D` (`self.Bounds`))))
  (`|ExecutionSequence`
    (:`then_0`
      (`self.VolumeDataAsset`
        (:`then`)
        (:`else`
          (bind _returnvalue (`|GenericCreateObject` self "/TAToolsPlugin/ShallowWater/Material30/Tools/DistanceField/Blueprints/PDA_FluxSignedDistanceField.PDA_FluxSignedDistanceField_C"))
          (set `self.VolumeDataAsset` _returnvalue))))
    (:`then_1`
      (`self.VolumeDataAsset`
        (:`then`
          (`/TAToolsPlugin/ShallowWater/Material30/Tools/DistanceField/Blueprints/PDA_FluxSignedDistanceField.SetData` (`self.VolumeDataAsset`) (`self.SignedDistanceField`) (`KismetMathLibrary.MakeVector` _relativescale3d_y _relativescale3d_z) (`KismetMathLibrary.MakeVector` _relativelocation_y _relativelocation_z) (make `IntPoint` 1 1) (`self.DistanceRange`)))
        (:`else`)))
    (:`then_2`
      (return))))

(fn `InitializeDebug`
  (`self.DebugInstance`
    (:`then`
      _)
    (:`else`
      (bind _returnvalue (`PrimitiveComponent.CreateDynamicMaterialInstance` (`self.DebugPreview`) 0 null "None"))
      (bind _output_get (set `self.DebugInstance` _returnvalue))))
  (`/TAToolsPlugin/ShallowWater/Material30/Tools/DistanceField/Blueprints/PDA_FluxSignedDistanceField.ApplyMaterialParameters` (`self.VolumeDataAsset`) (`|MakeArray` _output_get) "" false))

(fn `InitializeMesh`
  (`self.CrossectionInstance`
    (:`then`
      _)
    (:`else`
      (bind _returnvalue (`KismetMaterialLibrary.CreateDynamicMaterialInstance` "/TAToolsPlugin/ShallowWater/Material30/Tools/DistanceField/Materials/M_SDFMeshCrossection.M_SDFMeshCrossection"))
      (set `self.CrossectionInstance` _returnvalue)))
  (`StaticMeshComponent.SetStaticMesh` (`self.StaticMesh`) (`self.CapturedMesh`))
  (`MaterialInstanceDynamic.SetScalarParameterValue` (`self.CrossectionInstance`) "Range" (`self.DistanceRange`))
  (for _index (range (`PrimitiveComponent.GetNumMaterials` (`self.StaticMesh`)))
    (`PrimitiveComponent.SetMaterial` (`self.StaticMesh`) _index (`self.CrossectionInstance`))))

(fn `InitializeRenderTargets`
  (bind _textureresolution (`self.TextureResolution`))
  (bind (_returnvalue _newtexture) (`/Game/FluidFlux20/Editor/Blueprints/BPL_FluidFlux.RecreateRenderTarget` _textureresolution _textureresolution (select `bool` (`self.HighPrecission`) :`false` "RTF_R8" :`true` "RTF_R16f" :!type "ETextureRenderTargetFormat Enum") (struct :`R` 1.0 :`G` 1.0 :`B` 1.0 :`A` 1.0) null (`self.SignedDistanceField`)))
  (set `self.SignedDistanceField` _newtexture)
  (set `Texture.SRGB` false _newtexture))

(fn `InitializeSceneCapture`
  (locals (Bounds :type "Vector Structure") (Offset :type "Vector Structure" :default (0.0 0.0 0.0)))
  (bind (_bounds_x _bounds_y _bounds_z) (`KismetMathLibrary.BreakVector` (`local.Bounds`)))
  (bind (_offset_x _offset_y _offset_z) (`KismetMathLibrary.BreakVector` (`local.Offset`)))
  (bind (_offset_x_2 _offset_y_2 _offset_z_2) (`KismetMathLibrary.BreakVector` (`local.Offset`)))
  (bind (_bounds_x_2 _bounds_y_2 _bounds_z_2) (`KismetMathLibrary.BreakVector` (`local.Bounds`)))
  (bind (_canvasoffset_x _canvasoffset_y) (`KismetMathLibrary.BreakVector2D` (`self.CanvasOffset`)))
  (bind (_bounds_x_3 _bounds_y_3 _bounds_z_3) (`KismetMathLibrary.BreakVector` (`local.Bounds`)))
  (bind (_offset_x_3 _offset_y_3 _offset_z_3) (`KismetMathLibrary.BreakVector` (`local.Offset`)))
  (bind (_min _max) (`StaticMeshComponent.GetLocalBounds` (`self.StaticMesh`)))
  (bind (_min_2 _max_2) (`StaticMeshComponent.GetLocalBounds` (`self.StaticMesh`)))
  (bind _returnvalue (`KismetMathLibrary.FMax` _bounds_y_2 _bounds_z_2))
  (set `SceneCaptureComponent.ShowOnlyActors` (`|MakeArray` self :!type "Actor Object Reference") (`self.SceneCaptureComponent2D`))
  (set `SceneCaptureComponent2D.TextureTarget` (`self.SignedDistanceField`) (`self.SceneCaptureComponent2D`))
  (set `local.Bounds` (+ (- _max _min) (* (`self.DistanceRange`) (`self.CanvasScale`))))
  (set `local.Bounds` (`KismetMathLibrary.MakeVector` 10.0 _returnvalue _returnvalue))
  (`SceneComponent.SetRelativeScale3D` (`self.Bounds`) (`local.Bounds`))
  (set `local.Offset` (+ (`KismetMathLibrary.VLerp` _min_2 _max_2 0.5) (`KismetMathLibrary.MakeVector` 0.0 _canvasoffset_x _canvasoffset_y)))
  (`SceneComponent.K2_SetRelativeLocation` (`self.Bounds`) (`KismetMathLibrary.MakeVector` 0.0 _offset_y _offset_z) false false)
  (`SceneComponent.K2_SetRelativeLocation` (`self.SceneCaptureComponent2D`) (`KismetMathLibrary.MakeVector` -10.0 _offset_y_2 _offset_z_2) false false)
  (set `SceneCaptureComponent2D.OrthoWidth` (`KismetMathLibrary.FMax` _bounds_y _bounds_z) (`self.SceneCaptureComponent2D`))
  (bind _debugpreview (`self.DebugPreview`)
    (:`then`
      (`SceneComponent.K2_SetRelativeTransform` _debugpreview (`KismetMathLibrary.MakeTransform` (`KismetMathLibrary.MakeVector` -20.0 _offset_y_3 _offset_z_3) (struct :`Yaw` 90.0 :`Roll` 90.0) (* (`KismetMathLibrary.MakeVector` _bounds_z_3 _bounds_y_3 1.0) 0.01)) false false))
    (:`else`)))

(fn `Repaint`
  (`SceneCaptureComponent2D.CaptureScene` (`self.SceneCaptureComponent2D`))
  (if (`self.UseJumpFood`)
    (set `/TAToolsPlugin/ShallowWater/Material30/Tools/DistanceField/Blueprints/BP_FluxJumpFloodComponent.Result` (`self.SignedDistanceField`) (`self.JumpFloodComponent`))
    (`/TAToolsPlugin/ShallowWater/Material30/Tools/DistanceField/Blueprints/BP_FluxJumpFloodComponent.Generate` (`self.JumpFloodComponent`) (`self.SignedDistanceField`) (`self.Normalization`) true (`self.DistanceFieldEdgeIterations`) 0.5)))

(fn `UserConstructionScript`
  (set `self.TextureResolution` (`KismetMathLibrary.FTrunc` (`KismetMathLibrary.MultiplyMultiply_FloatFloat` 2.0 (`KismetMathLibrary.Conv_IntToDouble` (`KismetMathLibrary.Round` (`KismetMathLibrary.Log` (`KismetMathLibrary.Conv_IntToDouble` (`self.TextureResolution`)) 2.0))))))
  (`self.InitializeAll`)
  (`self.Repaint`))