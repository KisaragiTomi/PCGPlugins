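; BP_SDFShape is a placeable analytic shape that feeds signed distance field capture in the ShallowWater tools.
; It returns an SDF shape built from actor location, rotation, Size and Round, along with a fixed source type.
; Construction locks scale to one and triggers CaptureDistanceFields on every BP_SDFVolumeDomain.
; It adds a box component sized by Size, or a sphere when Round equals Size.X.
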(fn `GetShapes`
  (returns (Shapes :type "Array of /TAToolsPlugin/ShallowWater/Material30/Tools/DistanceField/Blueprints/BS_SDFShape Structure"))
  (return (`|MakeArray` (make `/TAToolsPlugin/ShallowWater/Material30/Tools/DistanceField/Blueprints/BS_SDFShape` (`KismetMathLibrary.MakeTransform` (`self.K2_GetActorLocation`) (`self.K2_GetActorRotation`) (`self.Size`)) (`self.Round`)))))

(fn `GetSourceType`
  (returns (Type :type "/TAToolsPlugin/ShallowWater/Material30/Tools/DistanceField/Blueprints/BPE_SDFSourceType Enum"))
  (return "NewEnumerator0"))

(fn `RefreshSurfaceData`
  (bind _outactors (`GameplayStatics.GetAllActorsOfClass` "/TAToolsPlugin/ShallowWater/Material30/Tools/DistanceField/Blueprints/BP_SDFVolumeDomain.BP_SDFVolumeDomain_C"))
  (for _array_element _outactors
    (`/TAToolsPlugin/ShallowWater/Material30/Tools/DistanceField/Blueprints/BP_SDFVolumeDomain.CaptureDistanceFields` _array_element)))

(fn `UserConstructionScript`
  (bind _size_x (`KismetMathLibrary.BreakVector` (`self.Size`)))
  (`self.SetActorScale3D` (1.0 1.0 1.0))
  (`self.RefreshSurfaceData`)
  (if (!= (`self.Round`) _size_x)
    (bind _returnvalue (`AddComponent|NODE_AddBoxComponent-0`))
    (`BoxComponent.SetBoxExtent` _returnvalue (`self.Size`) true)
    (else
      (bind _returnvalue_2 (`AddComponent|NODE_AddSphereComponent-0`))
      (`SphereComponent.SetSphereRadius` _returnvalue_2 (`self.Round`) true))))