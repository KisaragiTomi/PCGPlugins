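; Volume actor that bakes source actors into a signed distance field, stored as a tiled 2D render-target atlas of Z slices.
; Captures on begin play, construction, source change or tick, using Niagara if available, otherwise material draws.
; The material path ping-pongs two targets, drawing heightmaps whole and splines per slice, ending in texture A.
; A data asset passes the volume to FluxSurface and SDFRenderer targets after full captures.
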(event `self.ReceiveBeginPlay`
  (if (`self.AffectWorld`)
    (`self.InitializeAll`)
    (`KismetSystemLibrary.Delay` 0.2)
    (`self.CaptureDistanceFields`)))

(event `Capture`
  (if (`self.AffectWorld`)
    (`KismetSystemLibrary.K2_SetTimer` null "CaptureDistanceFields" (`self.RuntimeCaptureDelay`))))

(event `/TAToolsPlugin/ShallowWater/Material30/Tools/DistanceField/Blueprints/BPI_SDFVolume.OnCapturedShapeChanged`
  (params (Source :type "Actor Object Reference"))
  (if (`self.AffectWorld`)
    (if (>= (`KismetArrayLibrary.Array_Find` (`self.SourceActors`) Source) 0)
      (`self.CaptureDistanceFields`))))

(event `self.ReceiveTick`
  (params (DeltaSeconds :type "Float (single-precision)"))
  (`self.NiagaraRasterizer`
    (:`then`
      (`self.CaptureWithNiagara`))
    (:`else`
      (`self.CaptureWithBlueprints`))))

(fn `ApplyToActors`
  (locals (PreviewActor :type "Actor Object Reference"))
  (if (`self.AffectWorld`)
    (for _array_element (`self.TargetActors`)
      (set `local.PreviewActor` _array_element)
      (`|ExecutionSequence`
        (:`then_0`
          (if (`KismetSystemLibrary.DoesImplementInterface` (`local.PreviewActor`) "/TAToolsPlugin/ShallowWater/Material30/Surface/Blueprints/BPI_FluxSurface.BPI_FluxSurface_C")
            (message `/TAToolsPlugin/ShallowWater/Material30/Surface/Blueprints/BPI_FluxSurface.SetSignedDistanceFieldMask` (`local.PreviewActor`) (`self.VolumeDataAsset`))))
        (:`then_1`
          (if (`KismetSystemLibrary.DoesImplementInterface` (`local.PreviewActor`) "/TAToolsPlugin/ShallowWater/Material30/Tools/DistanceField/Blueprints/BPI_SDFRenderer.BPI_SDFRenderer_C")
            (message `/TAToolsPlugin/ShallowWater/Material30/Tools/DistanceField/Blueprints/BPI_SDFRenderer.ApplySignedDistanceField` (`local.PreviewActor`) (`self.VolumeDataAsset`))))))
    (`self.Debug`
      (:`then`
        (`/TAToolsPlugin/ShallowWater/Material30/Tools/DistanceField/Blueprints/PDA_FluxSignedDistanceField.ApplyMaterialParameters` (`self.VolumeDataAsset`) (`|MakeArray` (`self.DebugMaterial`)) "" false))
      (:`else`))))

(fn `CaptureDistanceFields`
  (locals (CapturedActor :type "Actor Object Reference") (PreviewActor :type "Actor Object Reference"))
  (`|ExecutionSequence`
    (:`then_0`
      (`self.NiagaraRasterizer`
        (:`then`
          (`self.CaptureWithNiagara`))
        (:`else`
          (`self.CaptureWithBlueprints`))))
    (:`then_1`
      (`self.ApplyToActors`))))

(fn `CaptureWithBlueprints`
  (locals (CapturedActor :type "Actor Object Reference") (TileIndex :type Integer) (RenderToA :type Boolean))
  (bind (_resolution_x _resolution_y _resolution_z) (break `IntVector` (`self.Resolution`)))
  (bind _returnvalue (select `bool` (`self.Inverse`) :`true` (struct :`R` 1.0 :`G` 1.0 :`B` 1.0 :`A` 1.0) :!type "LinearColor Structure"))
  (`KismetRenderingLibrary.ClearRenderTarget2D` (`self.VolumeTextureA`) _returnvalue)
  (`KismetRenderingLibrary.ClearRenderTarget2D` (`self.VolumeTextureB`) _returnvalue)
  (set `local.RenderToA` (`KismetMathLibrary.Conv_IntToBool` (mod (`KismetArrayLibrary.Array_Length` (`self.SourceActors`)) 2)))
  (for _array_element (`self.SourceActors`)
    (set `local.CapturedActor` _array_element)
    (bind _capturedactor (`local.CapturedActor`)
      (:`then`
        (bind _type (message `/TAToolsPlugin/ShallowWater/Material30/Tools/DistanceField/Blueprints/BPI_SDFSource.GetSourceType` _capturedactor))
        (switch `/TAToolsPlugin/ShallowWater/Material30/Tools/DistanceField/Blueprints/BPE_SDFSourceType` _type
          (:`NewEnumerator1`
            (message `/TAToolsPlugin/ShallowWater/Material30/Tools/DistanceField/Blueprints/BPI_SDFSource.PrepareMaterial` (`local.CapturedActor`) (`self.SDFHeightmapInstance`))
            (bind (_flag _source _target) (`self.SwitchBffers` (`local.RenderToA`)))
            (set `local.RenderToA` _flag)
            (`MaterialInstanceDynamic.SetTextureParameterValue` (`self.SDFHeightmapInstance`) "SDFPrevious" _source)
            (`KismetRenderingLibrary.DrawMaterialToRenderTarget` _target (`self.SDFHeightmapInstance`)))
          (:`NewEnumerator0`
            (bind _shapes (message `/TAToolsPlugin/ShallowWater/Material30/Tools/DistanceField/Blueprints/BPI_SDFSource.GetShapes` (`local.CapturedActor`))))
          (:`NewEnumerator3`
            (message `/TAToolsPlugin/ShallowWater/Material30/Tools/DistanceField/Blueprints/BPI_SDFSource.PrepareMaterial` (`local.CapturedActor`) (`self.SDFTileInstance`))
            (bind (_flag_2 _source_2 _target_2) (`self.SwitchBffers` (`local.RenderToA`)))
            (set `local.RenderToA` _flag_2)
            (`MaterialInstanceDynamic.SetTextureParameterValue` (`self.SDFTileInstance`) "SDFPrevious" _source_2)
            (for _index (range _resolution_z)
              (set `local.TileIndex` _index)
              (message `/TAToolsPlugin/ShallowWater/Material30/Tools/DistanceField/Blueprints/BPI_SDFSource.Capture` (`local.CapturedActor`) (`/TAToolsPlugin/ShallowWater/Material30/Tools/DistanceField/Blueprints/PDA_FluxSignedDistanceField.GetLayerZLocation` (`self.VolumeDataAsset`) (`local.TileIndex`)))
              (`MaterialInstanceDynamic.SetScalarParameterValue` (`self.SDFTileInstance`) "FrameIndex" (`KismetMathLibrary.Conv_IntToDouble` (`local.TileIndex`)))
              (`KismetRenderingLibrary.DrawMaterialToRenderTarget` _target_2 (`self.SDFTileInstance`))))))
      (:`else`)))
  ;[0.5203 0.8438 1] Flip last to write into A
  (if (`local.RenderToA`)
    (`MaterialInstanceDynamic.SetTextureParameterValue` (`self.SDFInverseInstance`) "SDFPrevious" (`self.VolumeTextureB`))
    (`KismetRenderingLibrary.DrawMaterialToRenderTarget` (`self.VolumeTextureA`) (`self.SDFInverseInstance`))
    (`KismetRenderingLibrary.ClearRenderTarget2D` (`self.VolumeTextureB`))
    (else
      (`KismetRenderingLibrary.ClearRenderTarget2D` (`self.VolumeTextureB`)))))

(fn `CaptureWithNiagara`
  (locals (ShapeLocationRadius :type "Array of Vector4 Structure") (ShapeSize :type "Array of Vector Structure") (ShapeRotation :type "Array of Quat Structure") (ShapeForward :type "Array of Vector Structure") (ShapeUp :type "Array of Vector Structure"))
  (`self.NiagaraRasterizer`
    (:`then`
      (`|ExecutionSequence`
        (:`then_1`
          (`NiagaraDataInterfaceArrayFunctionLibrary.SetNiagaraArrayVector4` (`self.NiagaraRasterizer`) "ShapeLocationRadius" (`local.ShapeLocationRadius`))
          (`NiagaraDataInterfaceArrayFunctionLibrary.SetNiagaraArrayVector` (`self.NiagaraRasterizer`) "ShapeSize" (`local.ShapeSize`))
          (`NiagaraDataInterfaceArrayFunctionLibrary.SetNiagaraArrayVector` (`self.NiagaraRasterizer`) "ShapeForward" (`local.ShapeForward`))
          (`NiagaraDataInterfaceArrayFunctionLibrary.SetNiagaraArrayVector` (`self.NiagaraRasterizer`) "ShapeUp" (`local.ShapeUp`)))
        (:`then_2`
          (`NiagaraComponent.AdvanceSimulation` (`self.NiagaraRasterizer`) 1 1.0))))
    (:`else`)))

(fn `GetShapeParameters`
  (params (BS_SDFShape :type "/TAToolsPlugin/ShallowWater/Material30/Tools/DistanceField/Blueprints/BS_SDFShape Structure (by ref)"))
  (returns (LocationRadius :type "LinearColor Structure") (Size :type "LinearColor Structure") (Forward :type "LinearColor Structure") (Up :type "LinearColor Structure"))
  (bind (_transform _radius) (break `/TAToolsPlugin/ShallowWater/Material30/Tools/DistanceField/Blueprints/BS_SDFShape` BS_SDFShape))
  (bind _returnvalue (`KismetMathLibrary.NegateRotator` (.rotation _transform)))
  (return (`KismetMathLibrary.MakeColor` (.x (.location _transform)) (.y (.location _transform)) (.z (.location _transform)) _radius) (`KismetMathLibrary.Conv_VectorToLinearColor` (.scale _transform)) (`KismetMathLibrary.Conv_VectorToLinearColor` (`KismetMathLibrary.GetForwardVector` _returnvalue)) (`KismetMathLibrary.Conv_VectorToLinearColor` (`KismetMathLibrary.GetUpVector` _returnvalue))))

(fn `InitializeAll`
  (`|ExecutionSequence`
    (:`then_0`
      (`self.InitializeRenderTargets`))
    (:`then_1`
      (`self.InitializeArea`))
    (:`then_2`
      (`self.InitlializeBlueprintRasterizer`))
    (:`then_3`
      (`self.InitializeNiagaraRasterizer`))
    (:`then_4`
      (`self.Set Update Frequency` (`self.UpdateFrequency`)))))

(fn `InitializeArea`
  (bind (_worldtexelsize_x _worldtexelsize_y _worldtexelsize_z) (`KismetMathLibrary.BreakVector` (`self.WorldTexelSize`)))
  (`|ExecutionSequence`
    (:`then_0`
      (set `self.WorldTexelSize` (`KismetMathLibrary.MakeVector` _worldtexelsize_x _worldtexelsize_x _worldtexelsize_z))
      (set `self.VolumeSize` (* (`self.WorldTexelSize`) (`self.Resolution`)))
      (`SceneComponent.SetRelativeScale3D` (`self.Bounds`) (`self.VolumeSize`))
      (`self.K2_SetActorRotation` (struct)))
    (:`then_1`
      (`self.VolumeDataAsset`
        (:`then`)
        (:`else`
          (bind _returnvalue (`|GenericCreateObject` self "/TAToolsPlugin/ShallowWater/Material30/Tools/DistanceField/Blueprints/PDA_FluxSignedDistanceField.PDA_FluxSignedDistanceField_C"))
          (set `self.VolumeDataAsset` _returnvalue))))
    (:`then_2`
      (`self.VolumeDataAsset`
        (:`then`
          (`/TAToolsPlugin/ShallowWater/Material30/Tools/DistanceField/Blueprints/PDA_FluxSignedDistanceField.SetData` (`self.VolumeDataAsset`) (`self.VolumeTextureA`) (`self.VolumeSize`) (`SceneComponent.K2_GetComponentLocation` (`self.Bounds`)) (`self.Tiles`) (`KismetMathLibrary.SelectFloat` (* (`self.DistanceRange`) -1.0) (`self.DistanceRange`))))
        (:`else`)))
    (:`then_3`
      (bind _debug (`self.Debug`)
        (:`then`
          (`SceneComponent.SetRelativeScale3D` _debug (* (`self.VolumeSize`) 0.01))
          (bind _returnvalue_2 (`PrimitiveComponent.CreateDynamicMaterialInstance` _debug 0 null "None"))
          (set `self.DebugMaterial` _returnvalue_2))
        (:`else`)))))

(fn `InitializeNiagaraRasterizer`
  (`self.NiagaraSystem`
    (:`then`
      (`|ExecutionSequence`
        (:`then_0`
          (`self.NiagaraRasterizer`
            (:`then`)
            (:`else`
              (bind _returnvalue (`AddComponent|NODE_AddNiagaraComponent-0`))
              (bind _output_get (set `self.NiagaraRasterizer` _returnvalue))
              (`NiagaraComponent.SetAsset` _output_get (`self.NiagaraSystem`) true))))
        (:`then_1`
          (`NiagaraComponent.SetAgeUpdateMode` (`self.NiagaraRasterizer`) "DesiredAgeNoSeek")
          (`NiagaraComponent.SetLockDesiredAgeDeltaTimeToSeekDelta` (`self.NiagaraRasterizer`) true))
        (:`then_2`
          (`/TAToolsPlugin/ShallowWater/Material30/Tools/DistanceField/Blueprints/PDA_FluxSignedDistanceField.ApplyNiagaraParameters` (`self.VolumeDataAsset`) (`self.NiagaraRasterizer`)))))
    (:`else`)))

(fn `InitializeRenderTargets`
  (locals (TilesY :type Integer :default 0) (TilesX :type Integer :default 0))
  (bind (_tiles_x _tiles_y) (break `IntPoint` (`self.Tiles`)))
  (bind (_resolution_x _resolution_y) (break `IntVector` (`self.Resolution`)))
  (bind (_resolution_x_2 _resolution_y_2 _resolution_z) (break `IntVector` (`self.Resolution`)))
  (bind (_resolution_x_3 _resolution_y_3) (break `IntVector` (`self.Resolution`)))
  (bind (_tiles_x_2 _tiles_y_2) (break `IntPoint` (`self.Tiles`)))
  (set `self.Tiles` (`self.FramesToTiles` _resolution_z))
  (`|ExecutionSequence`
    (:`then_0`
      (bind (_returnvalue _newtexture) (`/Game/FluidFlux20/Editor/Blueprints/BPL_FluidFlux.RecreateRenderTarget` (* _tiles_x_2 _resolution_x_3) (* _tiles_y_2 _resolution_y_3) (select `bool` (`self.HighPrecission`) :`false` "RTF_R8" :`true` "RTF_R16f" :!type "ETextureRenderTargetFormat Enum") (struct :`R` 1.0 :`G` 1.0 :`B` 1.0 :`A` 1.0) null (`self.VolumeTextureA`)))
      (bind _output_get (set `self.VolumeTextureA` _newtexture))
      (set `Texture.SRGB` false _output_get))
    (:`then_1`
      (bind (_returnvalue_2 _newtexture_2) (`/Game/FluidFlux20/Editor/Blueprints/BPL_FluidFlux.RecreateRenderTarget` (* _tiles_x _resolution_x) (* _tiles_y _resolution_y) (select `bool` (`self.HighPrecission`) :`false` "RTF_R8" :`true` "RTF_R16f" :!type "ETextureRenderTargetFormat Enum") (struct :`R` 1.0 :`G` 1.0 :`B` 1.0 :`A` 1.0) null (`self.VolumeTextureB`)))
      (bind _output_get_2 (set `self.VolumeTextureB` _newtexture_2))
      (set `Texture.SRGB` false _output_get_2))))

(fn `InitlializeBlueprintRasterizer`
  (`KismetArrayLibrary.Array_Clear` (`self.SDFInstances`))
  (`|ExecutionSequence`
    (:`then_0`
      (`self.SDFShapeInstance`
        (:`then`
          _)
        (:`else`
          (bind _returnvalue (`KismetMaterialLibrary.CreateDynamicMaterialInstance` "/TAToolsPlugin/ShallowWater/Material30/Tools/DistanceField/Materials/MI_RenderSDFShape.MI_RenderSDFShape"))
          (set `self.SDFShapeInstance` _returnvalue)))
      (`KismetArrayLibrary.Array_Add` (`self.SDFInstances`) (`self.SDFShapeInstance`)))
    (:`then_1`
      (`self.SDFHeightmapInstance`
        (:`then`
          _)
        (:`else`
          (bind _returnvalue_2 (`KismetMaterialLibrary.CreateDynamicMaterialInstance` "/TAToolsPlugin/ShallowWater/Material30/Tools/DistanceField/Materials/MI_RenderSDFHeightnap.MI_RenderSDFHeightnap"))
          (set `self.SDFHeightmapInstance` _returnvalue_2)))
      (`KismetArrayLibrary.Array_Add` (`self.SDFInstances`) (`self.SDFHeightmapInstance`)))
    (:`then_2`
      (`self.SDFTileInstance`
        (:`then`
          _)
        (:`else`
          (bind _returnvalue_3 (`KismetMaterialLibrary.CreateDynamicMaterialInstance` "/TAToolsPlugin/ShallowWater/Material30/Tools/DistanceField/Materials/M_RenderSDFTile.M_RenderSDFTile"))
          (set `self.SDFTileInstance` _returnvalue_3)))
      (`KismetArrayLibrary.Array_Add` (`self.SDFInstances`) (`self.SDFTileInstance`)))
    (:`then_3`
      (`self.SDFInverseInstance`
        (:`then`
          _)
        (:`else`
          (bind _returnvalue_4 (`KismetMaterialLibrary.CreateDynamicMaterialInstance` "/TAToolsPlugin/ShallowWater/Material30/Tools/DistanceField/Materials/M_InverseCopySDF.M_InverseCopySDF"))
          (set `self.SDFInverseInstance` _returnvalue_4)))
      (`KismetArrayLibrary.Array_Add` (`self.SDFInstances`) (`self.SDFInverseInstance`)))
    (:`then_4`
      (`/TAToolsPlugin/ShallowWater/Material30/Tools/DistanceField/Blueprints/PDA_FluxSignedDistanceField.ApplyMaterialParameters` (`self.VolumeDataAsset`) (`self.SDFInstances`) "" false)
      (`MaterialInstanceDynamic.SetScalarParameterValue` (`self.SDFInstances`) "SDFInverse" (`KismetMathLibrary.Conv_BoolToDouble` (`self.Inverse`))))))

(fn `Set Update Frequency`
  (params (Interval :type "Float (double-precision)"))
  (bind _output_get (set `self.UpdateFrequency` Interval))
  (if (>= _output_get 0.0)
    (`self.SetActorTickInterval` (`self.UpdateFrequency`))
    (`self.SetActorTickEnabled` true)
    (else
      (`self.SetActorTickEnabled` false))))

(fn `SwitchBffers`
  (params (Index :type Boolean))
  (returns (Flag :type Boolean) (Source :type "Texture Object Reference") (Target :type "TextureRenderTarget2D Object Reference"))
  (return (not Index) (select `bool` Index :`false` (`self.VolumeTextureA`) :`true` (`self.VolumeTextureB`) :!type "Texture Object Reference") (select `bool` Index :`false` (`self.VolumeTextureB`) :`true` (`self.VolumeTextureA`))))

(fn `UserConstructionScript`
  (if (`self.AffectWorld`)
    (`self.InitializeAll`)
    (`self.Capture`)))