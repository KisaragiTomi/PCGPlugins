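; Primary data asset for the Flux shallow water tools that stores a signed distance field texture with its position, size, tile grid and distance range.
; It pushes these to ID-suffixed material parameters, packing range into size alpha (negated when inverted), and to FluxSDF Niagara parameters.
; The texture tiles act as Z slices, with a helper mapping each layer index to world height.
; An event clears the texture reference.
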(event `self.ClearExternalReferences`
  (set `self.SignedDistanceField` null))

(fn `ApplyMaterialParameters`
  (params (MaterialInstances :type "Array of MaterialInstanceDynamic Object Reference") (ID :type String) (Inverse :type Boolean))
  (bind (_tiles_x _tiles_y) (break `IntPoint` (`self.Tiles`)))
  (bind (_size_x _size_y _size_z) (`KismetMathLibrary.BreakVector` (`self.Size`)))
  (bind _distancerange (`self.DistanceRange`))
  (`self.SignedDistanceField`
    (:`then`
      (`MaterialInstanceDynamic.SetTextureParameterValue` (`local.MaterialInstances`) (`KismetStringLibrary.Conv_StringToName` (`KismetStringLibrary.Concat_StrStr` "SDFMap" (`local.ID`))) (`self.SignedDistanceField`))
      (`MaterialInstanceDynamic.SetVectorParameterValue` (`local.MaterialInstances`) (`KismetStringLibrary.Conv_StringToName` (`KismetStringLibrary.Concat_StrStr` "SDFPosition" (`local.ID`))) (`KismetMathLibrary.Conv_VectorToLinearColor` (`self.Position`)))
      (`MaterialInstanceDynamic.SetVectorParameterValue` (`local.MaterialInstances`) (`KismetStringLibrary.Conv_StringToName` (`KismetStringLibrary.Concat_StrStr` "SDFSize" (`local.ID`))) (`KismetMathLibrary.MakeColor` _size_x _size_y _size_z (select `bool` (`local.Inverse`) :`false` _distancerange :`true` (* _distancerange -1.0) :!type "Float (single-precision)")))
      (`MaterialInstanceDynamic.SetVectorParameterValue` (`local.MaterialInstances`) (`KismetStringLibrary.Conv_StringToName` (`KismetStringLibrary.Concat_StrStr` "SDFTiles" (`local.ID`))) (`KismetMathLibrary.MakeColor` (`KismetMathLibrary.Conv_IntToDouble` _tiles_x) (`KismetMathLibrary.Conv_IntToDouble` _tiles_y) (`KismetMathLibrary.Conv_IntToDouble` (* _tiles_x _tiles_y)) 0.0)))
    (:`else`)))

(fn `ApplyNiagaraParameters`
  (params (NiagaraSystem :type "NiagaraComponent Object Reference"))
  (bind (_tiles_x _tiles_y) (break `IntPoint` (`self.Tiles`)))
  (`self.SignedDistanceField`
    (:`then`
      (`|ExecutionSequence`
        (:`then_0`
          (`NiagaraComponent.SetVariablePosition` (`local.NiagaraSystem`) "FluxSDFLocation" (`self.Position`))
          (`FXSystemComponent.SetVectorParameter` (`local.NiagaraSystem`) "FluxSDFSize" (`self.Size`))
          (`FXSystemComponent.SetFloatParameter` (`local.NiagaraSystem`) "FluxSDFRange" (`self.DistanceRange`))
          (`NiagaraComponent.SetVariableVec2` (`local.NiagaraSystem`) "FluxSDFTiles" (`KismetMathLibrary.MakeVector2D` (`KismetMathLibrary.Conv_IntToDouble` _tiles_x) (`KismetMathLibrary.Conv_IntToDouble` _tiles_y))))
        (:`then_1`
          (`self.SignedDistanceField`
            (:`then`
              (`NiagaraFunctionLibrary.SetTextureObject` (`local.NiagaraSystem`) "FluxSDFMap" (`self.SignedDistanceField`)))
            (:`else`)))))
    (:`else`)))

(fn `GetLayerZLocation`
  (params (Index :type Integer))
  (returns (ZLocation :type "Float (double-precision)"))
  (bind (_position_x _position_y _position_z) (`KismetMathLibrary.BreakVector` (`self.Position`)))
  (bind (_tiles_x _tiles_y) (break `IntPoint` (`self.Tiles`)))
  (bind (_size_x _size_y _size_z) (`KismetMathLibrary.BreakVector` (`self.Size`)))
  (return (+ (* (`KismetMathLibrary.Lerp` (- 0.0 _size_z) _size_z (/ (`KismetMathLibrary.Conv_IntToDouble` Index) (- (* _tiles_x _tiles_y) 1))) 0.5) _position_z)))

(fn `SetData`
  (params (Texture :type "Texture Object Reference") (Size :type "Vector Structure") (Position :type "Vector Structure") (Tiles :type "IntPoint Structure") (DistanceRange :type "Float (double-precision)" :default 1.0))
  (set `self.SignedDistanceField` Texture)
  (set `self.Size` Size)
  (set `self.Position` Position)
  (set `self.Tiles` Tiles)
  (set `self.DistanceRange` DistanceRange)
  (return))