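; Editor generator actor that builds a surface mesh from a Flux shallow-water simulation state and bakes it to a static mesh asset.
; Rebuilds take the state from the source actor or data asset, run BPFluxMeshGenerator at the chosen LOD and padding, then optionally simplify.
; The construction script snaps to the simulation area and switches preview between generator mesh, surface actor and static mesh.
; Saving updates the target asset or creates one, copying collision.
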(event `self.OnRebuildGeneratedMesh`
  (params (TargetMesh :type "DynamicMesh Object Reference"))
  (`self.CreateMesh` TargetMesh))

(fn `CreateMesh`
  (params (TargetMesh :type "DynamicMesh Object Reference"))
  (locals (TempMesh :type "DynamicMesh Object Reference"))
  (bind _tempmesh (`local.TempMesh`))
  (set `local.TempMesh` TargetMesh)
  (bind _state (`self.GetSimulationState`))
  (`/Engine/EditorBlueprintResources/StandardMacros.IsValid` _state
    (:`Is Valid`
      (set `self.SourceDataAsset` _state))
    (:`Is Not Valid`
      _))
  (`self.SourceDataAsset`
    (:`then`
      (bind _valid (`/TAToolsPlugin/ShallowWater/Material30/Simulation/Blueprints/PDA_FluxSimulationState.IsDefinied` (`self.SourceDataAsset`)))
      (if _valid
        (`self.K2_SetActorLocation` (`/TAToolsPlugin/ShallowWater/Material30/Simulation/Blueprints/PDA_FluxSimulationState.AreaLocation` (`self.SourceDataAsset`)))
        (bind (_meshout _triangles) (`/TAToolsPlugin/ShallowWater/Material30/Surface/Blueprints/BP_FluxMeshGenerator.BuildMesh` (`self.BP_FluxMeshGenerator`) (`self.SourceDataAsset`) (`KismetMathLibrary.Conv_ByteToInt` (`self.BaseLevelOfDetail`)) (`self.Edge Padding Depth`)))
        (bind (_triangles_2 _vertices _texcoords _normals _colors) (break `/TAToolsPlugin/ShallowWater/Material30/Tools/ProceduralMesh/BS_MeshDefinition` _meshout))
        (bind (_newtriangleindiceslist _returnvalue) (`GeometryScriptLibrary_MeshBasicEditFunctions.AppendBuffersToMesh` (`local.TempMesh`) (make `GeometryScriptSimpleMeshBuffers` :`Vertices` _vertices :`Normals` _normals :`UV0` _texcoords :`VertexColors` _colors :`Triangles` _triangles) 0 false null))
        (set `local.TempMesh` _returnvalue)
        (`|ExecutionSequence`
          (:`then_0`
            (if (> (`self.SimplifyTolerance`) 0.0)
              (bind _returnvalue_2 (`GeometryScriptLibrary_MeshSimplifyFunctions.ApplySimplifyToTolerance` (`local.TempMesh`) (`self.SimplifyTolerance`) (`self.SimplifyOptions`) null))
              (set `local.TempMesh` _returnvalue_2)))
          (:`then_1`
            (set `self.TriangleCount` (`DynamicMesh.GetTriangleCount` _tempmesh))
            (set `self.VertexCount` (`GeometryScriptLibrary_MeshQueryFunctions.GetVertexCount` _tempmesh))))))
    (:`else`)))

(fn `CreateStaticMeshAsset`
  (bind _returnvalue (`KismetTextLibrary.Conv_TextToString` (`|FormatText` "{PathSource}/{FullPath}" (`KismetMathLibrary.SelectString` (`KismetStringLibrary.Concat_StrStr` "/") "/Game" (> (`KismetStringLibrary.Len` (`self.Plugin`)) 0)) (`self.PathName`))))
  (set `self.SourceGeneratorKey` (`KismetGuidLibrary.Conv_GuidToString` (`KismetGuidLibrary.NewGuid`)))
  (bind _returnvalue_2 (`BaseDynamicMeshComponent.GetDynamicMesh` (`self.DynamicMeshComponent`)))
  (`KismetSystemLibrary.PrintString` _returnvalue) ; Print for debug
  (bind _uniqueassetpathandname (`GeometryScriptLibrary_CreateNewAssetFunctions.CreateUniqueNewAssetPathName` _returnvalue (`self.AssetName`) (struct) null)
    (:`Failure`
      (`KismetSystemLibrary.PrintString` "Failed to Create Asset Path"))
    (:`Success`
      (bind _returnvalue_3 (`GeometryScriptLibrary_CreateNewAssetFunctions.CreateNewStaticMeshAssetFromMesh` _returnvalue_2 _uniqueassetpathandname (make `GeometryScriptCreateNewStaticMeshAssetOptions` false false false (struct :`bLerpUVs` true :`PositionPrecision` -2147483648 :`NormalPrecision` -1 :`TangentPrecision` -1 :`KeepPercentTriangles` 1.0 :`FallbackTarget` "Auto" :`FallbackPercentTriangles` 1.0 :`FallbackRelativeError` 1.0) 0.0 true (`self.Collision Mode`)) null)
        (:`Failure`
          (`KismetSystemLibrary.PrintString` "Failed to Create New Asset"))
        (:`Success`
          (bind _output_get (set `self.TargetStaticMesh` _returnvalue_3))
          (`GeometryScriptLibrary_CollisionFunctions.SetStaticMeshCollisionFromComponent` _output_get (`self.DynamicMeshComponent`) (struct :`bEmitTransaction` true) (struct :`bMarkAsCustomized` true) null)
          (for (_array_element _array_index) (`MeshComponent.GetMaterials` (`self.DynamicMeshComponent`))
            (`StaticMesh.SetMaterial` (`self.TargetStaticMesh`) _array_index _array_element)))))))

(fn `GetSimulationState`
  (returns (State :type "/TAToolsPlugin/ShallowWater/Material30/Simulation/Blueprints/PDA_FluxSimulationState Object Reference"))
  (`self.SourceActor`
    (:`then`
      (if (`KismetSystemLibrary.DoesImplementInterface` (`self.SourceActor`) "/TAToolsPlugin/ShallowWater/Material30/Interaction/Blueprints/Interfaces/BPI_FluxInteractionRenderer.BPI_FluxInteractionRenderer_C")
        (bind _state (message `/TAToolsPlugin/ShallowWater/Material30/Interaction/Blueprints/Interfaces/BPI_FluxInteractionRenderer.GetSimulationState` (`self.SourceActor`)))
        (return _state)
        (elif (`KismetSystemLibrary.DoesImplementInterface` (`self.SourceActor`) "/TAToolsPlugin/ShallowWater/Material30/Simulation/Blueprints/BPI_FluxSimulationDomain.BPI_FluxSimulationDomain_C")
          (bind _state_2 (message `/TAToolsPlugin/ShallowWater/Material30/Simulation/Blueprints/BPI_FluxSimulationDomain.GetCurrentSimulationState` (`self.SourceActor`)))
          (return _state_2)
          (else
            (set `self.SourceActor` null)
            (return null)))))
    (:`else`
      (return null))))

(fn `Rebuild`
  (bind _returnvalue (`BaseDynamicMeshComponent.GetDynamicMesh` (`self.DynamicMeshComponent`)))
  (`DynamicMesh.Reset` _returnvalue)
  (`self.MarkForMeshRebuild` true))

(fn `SaveToStaticMeshAsset`
  (`self.TargetStaticMesh`
    (:`then`
      (bind _returnvalue (`BaseDynamicMeshComponent.GetDynamicMesh` (`self.DynamicMeshComponent`)))
      (`GeometryScriptLibrary_StaticMeshFunctions.CopyMeshToStaticMesh` _returnvalue (`self.TargetStaticMesh`) (make `GeometryScriptCopyMeshToAssetOptions` (`self.RecomputeNormals`) false true false false true false (`MeshComponent.GetMaterials` (`self.DynamicMeshComponent`)) _ true) (struct) true null
        (:`Success`
          (`GeometryScriptLibrary_CollisionFunctions.SetStaticMeshCollisionFromComponent` (`self.TargetStaticMesh`) (`self.DynamicMeshComponent`) (make `GeometryScriptSetSimpleCollisionOptions` true) (struct :`bMarkAsCustomized` true) null)
          (if (not (`/TAToolsPlugin/ShallowWater/Material30/Simulation/Blueprints/PDA_FluxSimulationState.Static` (`self.SourceDataAsset`)))
            (`EditorDialogLibrary.ShowMessage` "Saving Mesh To StaticMeshActor" "Mesh saved correctly! \n \nPlease note that the mesh was generated from a dynamically generated simulation state so may be inconsistent with simulation data applied to surface at runtime. \n \nIf you plan to use a static mesh with a surface actor then: \n \n1) Export the simulation state data asset. \n2) Set SimulationDomain->AffectWorld to false. \n3) Apply the new data asset in SurfaceActor->SimulationState." "Ok" "No")))))
    (:`else`
      (`self.CreateStaticMeshAsset`))))

(fn `UserConstructionScript`
  (`|ExecutionSequence`
    (:`then_0`
      (bind _state (`self.GetSimulationState`))
      (`/Engine/EditorBlueprintResources/StandardMacros.IsValid` _state
        (:`Is Valid`
          (set `self.SourceDataAsset` _state))
        (:`Is Not Valid`
          _))
      (bind _sourcedataasset (`self.SourceDataAsset`)
        (:`then`
          (`self.K2_SetActorLocation` (`/TAToolsPlugin/ShallowWater/Material30/Simulation/Blueprints/PDA_FluxSimulationState.AreaLocation` _sourcedataasset)))
        (:`else`)))
    (:`then_1`
      ;[0.1272 0.1344 0.1301 0.992] Target actor - Surface
      (`self.PreviewActor`
        (:`then`
          (`|ExecutionSequence`
            (:`then_0`
              (if (`KismetSystemLibrary.DoesImplementInterface` (`self.PreviewActor`) "/TAToolsPlugin/ShallowWater/Material30/Surface/Blueprints/BPI_FluxSurface.BPI_FluxSurface_C")
                (switch `/TAToolsPlugin/ShallowWater/Material30/Tools/ProceduralMesh/BE_FluxMeshGeneratorMode` (`self.PreviewMode`)
                  (:`NewEnumerator0`
                    (message `/TAToolsPlugin/ShallowWater/Material30/Surface/Blueprints/BPI_FluxSurface.SetGeneratorMode` (`self.PreviewActor`) null false))
                  (:`NewEnumerator1`
                    (message `/TAToolsPlugin/ShallowWater/Material30/Surface/Blueprints/BPI_FluxSurface.SetGeneratorMode` (`self.PreviewActor`) null true))
                  (:`NewEnumerator2`
                    (message `/TAToolsPlugin/ShallowWater/Material30/Surface/Blueprints/BPI_FluxSurface.SetGeneratorMode` (`self.PreviewActor`) (`self.TargetStaticMesh`) true)))))
            (:`then_1`
              (switch `/TAToolsPlugin/ShallowWater/Material30/Tools/ProceduralMesh/BE_FluxMeshGeneratorMode` (`self.PreviewMode`)
                (:`NewEnumerator2`
                  (bind _asstatic_mesh_actor (cast `StaticMeshActor` (`self.PreviewActor`)))
                  (bind _staticmeshcomponent (`StaticMeshActor.StaticMeshComponent` _asstatic_mesh_actor))
                  (`StaticMeshComponent.SetStaticMesh` _staticmeshcomponent (`self.TargetStaticMesh`))
                  (`PrimitiveComponent.SetMaterial` _staticmeshcomponent 0 (`self.PreviewMaterial`))
                  (`self.K2_SetActorTransform` (`self.PreviewActor`) (`self.GetTransform`) false false)
                  (`KismetArrayLibrary.Array_AddUnique` (`Actor.Tags` (`self.PreviewActor`)) "FluxHide"))))))
        (:`else`
          (switch `/TAToolsPlugin/ShallowWater/Material30/Tools/ProceduralMesh/BE_FluxMeshGeneratorMode` (`self.PreviewMode`)
            (:`NewEnumerator2`
              (bind _returnvalue (`AddComponent|NODE_AddStaticMeshComponent-0`))
              (bind _output_get (set `self.PreviewMeshComponent` _returnvalue))
              (`StaticMeshComponent.SetStaticMesh` _output_get (`self.TargetStaticMesh`))
              (`PrimitiveComponent.SetMaterial` _output_get 0 (`self.PreviewMaterial`)))))))
    (:`then_2`
      (switch `/TAToolsPlugin/ShallowWater/Material30/Tools/ProceduralMesh/BE_FluxMeshGeneratorMode` (`self.PreviewMode`)
        (:`NewEnumerator0`
          (`SceneComponent.SetVisibility` (`self.DynamicMeshComponent`) true false)
          (`PrimitiveComponent.SetMaterial` (`self.DynamicMeshComponent`) 0 (`self.PreviewMaterial`))
          (set `BaseDynamicMeshComponent.bExplicitShowWireframe` (`self.ShowWireframe`) (`self.DynamicMeshComponent`)))
        (:`NewEnumerator1`
          (`SceneComponent.SetVisibility` (`self.DynamicMeshComponent`) false false))
        (:`NewEnumerator2`
          (`SceneComponent.SetVisibility` (`self.DynamicMeshComponent`) false false))))))