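; BP_FluxWorldBrush is a placeable brush that paints a target value into one Flux painter canvas type, such as color, coast erase or wave scale.
; Construction keeps the actor yaw-only, asks all world painters to re-render, and updates two debug meshes showing hardness, roundness and canvas color.
; Draw skips painters of other canvas types, then passes shape and blend settings to the material and draws a rect at the actor's transform.
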(fn `Draw`
  (params (Material :type "MaterialInstanceDynamic Object Reference (by ref)") (Painter :type "/TAToolsPlugin/ShallowWater/Material30/Tools/ScenePainter/Blueprints/BP_FluxWorldPainterComponent Object Reference (by ref)"))
  (bind _targetvalue (`self.TargetValue`))
  (if (== (`/TAToolsPlugin/ShallowWater/Material30/Tools/ScenePainter/Blueprints/BP_FluxWorldPainterComponent.CanvasType` Painter) (`self.Canvas`))
    (`MaterialInstanceDynamic.SetScalarParameterValue` (`local.Material`) "Hardness" (`self.ShapeHardness`))
    (`MaterialInstanceDynamic.SetScalarParameterValue` (`local.Material`) "Radius" (`self.ShapeRoundness`))
    (`MaterialInstanceDynamic.SetVectorParameterValue` (`local.Material`) "BrushColor" (`KismetMathLibrary.MakeColor` _targetvalue _targetvalue _targetvalue (- 1.0 (`self.BlendAdditive`))))
    (`/TAToolsPlugin/ShallowWater/Material30/Tools/ScenePainter/Blueprints/BP_FluxWorldPainterComponent.DrawRect` (`local.Painter`) (`local.Material`) (`self.GetTransform`))))

(fn `Repaint`
  (bind _outactors (`GameplayStatics.GetAllActorsWithInterface` "/TAToolsPlugin/ShallowWater/Material30/Tools/ScenePainter/Blueprints/BPI_FluxWorldPainter.BPI_FluxWorldPainter_C"))
  (for _array_element _outactors
    (message `/TAToolsPlugin/ShallowWater/Material30/Tools/ScenePainter/Blueprints/BPI_FluxWorldPainter.RenderScenePainter` _array_element)))

(fn `UserConstructionScript`
  (bind (_returnvalue_roll _returnvalue_pitch _returnvalue_yaw) (`KismetMathLibrary.BreakRotator` (`SceneComponent.K2_GetComponentRotation` (`self.DefaultSceneRoot`))))
  (bind _returnvalue (select `/TAToolsPlugin/ShallowWater/Material30/Tools/ScenePainter/Blueprints/BE_WorldBrushType` (`self.Canvas`) :`NewEnumerator1` (0.3 0.1 0.0) :`NewEnumerator0` (0.0 0.3 0.1) :`NewEnumerator2` (0.2 0.0 0.0) :!type "Vector Structure"))
  (`SceneComponent.K2_SetWorldRotation` (`self.DefaultSceneRoot`) (`KismetMathLibrary.MakeRotator` 0.0 0.0 _returnvalue_yaw) false false)
  (`|ExecutionSequence`
    (:`then_0`
      (`self.Repaint`))
    (:`then_1`
      (`/Engine/EditorBlueprintResources/StandardMacros.IsValid` (`self.SM_DebugBig`)
        (:`Is Valid`
          (`SceneComponent.SetRelativeScale3D` (`self.SM_DebugSmall`) (`KismetMathLibrary.Conv_DoubleToVector` (- 1.0 (/ 1.0 (`self.ShapeHardness`)))))
          (`PrimitiveComponent.SetCustomPrimitiveDataFloat` (`self.SM_DebugBig`) 5 (`self.ShapeRoundness`))
          (`PrimitiveComponent.SetCustomPrimitiveDataFloat` (`self.SM_DebugSmall`) 5 (`self.ShapeRoundness`))
          (`PrimitiveComponent.SetCustomPrimitiveDataVector3` (`self.SM_DebugSmall`) 0 _returnvalue)
          (`PrimitiveComponent.SetCustomPrimitiveDataVector3` (`self.SM_DebugBig`) 0 (* _returnvalue 2.0)))))))