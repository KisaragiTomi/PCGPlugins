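; Shallow-water simulation capture actor that drives water surface and caustics decal visuals and wraps solver controls for stepping, stopping, baking and debug views.
; ConstructActor, run on solver start, prepares source and depth data, then shows either the result mesh with material instances or the simulation plane HISM.
; The simulation view feeds velocity-height and depth-wet render targets into dynamic water and decal materials, with sim center and size set on the water.
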(event Custom|Rest
  (Variables|Default|SetSwitchVisable false)
  (Class|CSShallowWaterCapture|Clean))

(event EventBeginPlay)

(event Collision|EventActorBeginOverlap
  (params (OtherActor :type Actor%20Object%20Reference)))

(event EventTick
  (params (DeltaSeconds :type Float%20%28single-precision%29)))

(event EventOnSolverStarted
  (CallFunction|ConstructActor))

(event EventSetMaterialParameter
  (bind _rt_resultdepthwet (Variables|Default|GetRT_ResultDepthWet))
  (Rendering|ClearRenderTarget2D _rt_resultdepthwet (Variables|/Script/Engine.TextureRenderTarget2D|GetClearColor _rt_resultdepthwet)))

(fn ConstructionScript
  (Rendering|SetCastShadow (Variables|Default|GetReusltMesh) false))

(fn BPSetHeight
  (Class|CSShallowWaterCapture|SetHeight))

(fn ConstructActor
  (bind _reusltmesh (Variables|Default|GetReusltMesh))
  (bind _simuvcenter (Variables|Default|GetSimUVCenter))
  (bind _simvishism (Variables|Default|GetSimVisHISM))
  (bind _rt_resultvelheight (Variables|Default|GetRT_ResultVelHeight))
  (bind _rt_resultdepthwet (Variables|Default|GetRT_ResultDepthWet))
  (Class|CSShallowWaterCapture|CheckandCreateTextureSWSourcePoint)
  (Class|CSShallowWaterCapture|CleanDepthWetConstruct)
  (Components|InstancedStaticMesh|ClearInstances _simvishism)
  (Components|StaticMesh|SetStaticMesh _simvishism "/PCGPlugins/ShallowWater/VelocityHeight/SM_SimWaterPlane.SM_SimWaterPlane")
  (Utilities|FlowControl|Sequence
    (:then_0
      (if (Variables|Default|GetSwitchVisable)
        (Rendering|SetVisibility (Variables|Default|GetSimVisHISM) false false)
        (Rendering|SetVisibility _reusltmesh true false)
        (Rendering|Material|SetMaterial _reusltmesh 0 (Variables|Default|GetMI_WaterMaterial))
        (Rendering|Components|Decal|SetDecalMaterial (Variables|Default|GetCausticsDecal) (Variables|Default|GetMI_DecalMaterial))
        (else
          (Utilities|FlowControl|Sequence
            (:then_0
              (bind _returnvalue (Rendering|Material|CreateDynamicMaterialInstance (Variables|Default|GetReusltMesh) 0 (Variables|Default|GetWaterMaterial) "None" :!class /Script/Engine.PrimitiveComponent))
              (Variables|Default|SetDM_WaterMaterial _returnvalue)
              (Rendering|Material|SetTextureParameterValue (Variables|Default|GetDM_WaterMaterial) "CSSW_VelHeight" _rt_resultvelheight)
              (Rendering|Material|SetTextureParameterValue (Variables|Default|GetDM_WaterMaterial) "CSSW_DepthWet" _rt_resultdepthwet)
              (Rendering|Material|SetMaterial (Variables|Default|GetSimVisHISM) 0 (Variables|Default|GetDM_WaterMaterial)))
            (:then_1
              (bind _returnvalue_2 (Rendering|Material|CreateDynamicMaterialInstance (Variables|Default|GetDecalMaterial) "None" "None" :!class /Script/Engine.KismetMaterialLibrary))
              (Variables|Default|SetDM_DecalMaterail _returnvalue_2)
              (Rendering|Material|SetTextureParameterValue (Variables|Default|GetDM_DecalMaterail) "CSSW_VelHeight" _rt_resultvelheight)
              (Rendering|Material|SetTextureParameterValue (Variables|Default|GetDM_DecalMaterail) "CSSW_DepthWet" _rt_resultdepthwet)
              (Rendering|Components|Decal|SetDecalMaterial (Variables|Default|GetCausticsDecal) (Variables|Default|GetDM_DecalMaterail)))))))
    (:then_1
      (Rendering|Material|SetVectorParameterValue (Variables|Default|GetDM_WaterMaterial) "CSSW_SimCenter" (Utilities|Struct|MakeLinearColor (.x _simuvcenter) (.y _simuvcenter) (Variables|Default|GetSimUVSize) 1.0) :!class /Script/Engine.MaterialInstanceDynamic))))

(fn DebugView
  (Class|KismetRenderingLibrary|RenderTargetCreateStaticTexture2DEditorOnly (Variables|Default|GetRT_DebugView) "Debug" "TC_HDR" "TMGS_FromTextureGroup"))

(fn SimMult
  (Class|CSShallowWaterCapture|ShallowWaterSolverSoucePoint (Variables|Default|GetIteration)))

(fn CollisionPlane
  (Class|CSShallowWaterCapture|ShowDebugViewPlane 5.0))

(fn Sim
  (Class|CSShallowWaterCapture|ToggleSimVisualization 5))

(fn Test)

(fn SWSolverSingle
  (Class|CSShallowWaterCapture|ShallowWaterSolverSoucePoint 1))

(fn Bake
  (Class|CSShallowWaterCapture|BakeResultMesh))

(fn Stop
  (Class|CSShallowWaterCapture|StopSolver))