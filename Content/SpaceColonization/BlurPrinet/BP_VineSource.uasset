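; Vine source actor that previews space-colonization vines on a dynamic mesh and converts their tube, plane and target instances between scene foliage and transform arrays.
; VisVineExcute rebuilds the preview through two VisVine passes; foliage import first zeroes the actor's location and repositions its billboard.
; The construction script clears the mesh and attached actors, then configures bounds, foliage types and noise settings.
; Older generation and static-mesh baking chains remain disconnected.
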(event Custom|BP_CovnerInstance
  (Development|SetHiddeninGame (Variables|DynamicMeshActor|GetDynamicMeshComponent) false false)
  (Utilities|FlowControl|Sequence
    (:then_0
      (Class|VineContainer|ExportTransformArraytoFoliage (Variables|Default|GetTubeVineType)))
    (:then_1
      (Class|VineContainer|ExportTransformArraytoFoliage (Variables|Default|GetPlaneVineType)))
    (:then_2
      (Class|VineContainer|ExportTransformArraytoFoliage (Variables|Default|GetTargetInstances)))))

(event Custom|VisVineExcute
  (Development|SetHiddeninGame (Variables|DynamicMeshActor|GetDynamicMeshComponent) false false)
  (bind _returnvalue (DynamicMeshComponent|GetDynamicMesh (Variables|DynamicMeshActor|GetDynamicMeshComponent)))
  (DynamicMesh|Reset _returnvalue)
  (Utilities|FlowControl|Sequence
    (:then_0
      (Class|VineContainer|VisVine false))
    (:then_1
      (Class|VineContainer|VisVine true))))

(event Custom|BP_CraeteMesh
  (params (PathName :type String) (TubeMaterial :type Material%20Object%20Reference) (PlaneMaterial :type Material%20Object%20Reference)))

(event Custom|BP_ConvertFoliage
  (bind _billboard (Variables|Default|GetBillboard))
  (bind _output_get (Variables|Default|SetBillboardLocation (Transformation|GetWorldLocation _billboard)))
  (Transformation|SetActorLocation "0, 0, 0" false false)
  (Transformation|SetWorldLocation _billboard _output_get false false)
  (Utilities|FlowControl|Sequence
    (:then_0
      (Class|VineContainer|ImportFoliagetoTransformArray (Variables|Default|GetTubeVineType)))
    (:then_1
      (Class|VineContainer|ImportFoliagetoTransformArray (Variables|Default|GetPlaneVineType)))
    (:then_2
      (Class|VineContainer|ImportFoliagetoTransformArray (Variables|Default|GetTargetInstances)))))

(event Custom|Convert)

(event Custom|Test
  (Development|PrintString (Utilities|String|ToString(Integer) (Utilities|Array|Length (Variables|Default|GetGrowTargetTransforms)))))

(event EventBeginPlay)

(event Collision|EventActorBeginOverlap
  (params (OtherActor :type Actor%20Object%20Reference)))

(event EventTick
  (params (DeltaSeconds :type Float%20%28single-precision%29)))

(event EventCleanAll
  (Class|VineContainer|Clean))

(fn ConstructionScript
  (bind _dynamicmeshcomponent (Variables|DynamicMeshActor|GetDynamicMeshComponent))
  (bind _box_scale_3d (Variables|Default|GetBox%20Scale%203D))
  (Utilities|FlowControl|Sequence
    (:then_0
      (Utilities|FlowControl|Sequence
        (:then_0
          (bind _returnvalue (DynamicMeshComponent|GetDynamicMesh (Variables|DynamicMeshActor|GetDynamicMeshComponent)))
          (DynamicMesh|Reset _returnvalue))
        (:then_1
          (for _array_element (Actor|GetAttachedActors true false)
            (Actor|DestroyActor _array_element)))
        (:then_2
          (Development|SetHiddeninGame _dynamicmeshcomponent false false)
          (Rendering|Material|SetMaterial _dynamicmeshcomponent 0 (Variables|ViewEdit|GetTubeMaterial)))
        (:then_3
          (Transformation|SetRelativeScale3D (Variables|Default|GetGeneratorBounds) (Math|Vector|MakeVector _box_scale_3d _box_scale_3d _box_scale_3d)))))
    (:then_1
      (Variables|Default|SetTargetType "/PCGPlugins/SpaceColonization/SMF_Target_FoliageType.SMF_Target_FoliageType")
      (Variables|Default|SetTubeType "/PCGPlugins/SpaceColonization/SMF_TubeVine_FoliageType.SMF_TubeVine_FoliageType")
      (Variables|Default|SetPlaneType "/PCGPlugins/SpaceColonization/SMF_PlaneVine_FoliageType.SMF_PlaneVine_FoliageType")
      (Variables|Default|SetVV (Utilities|Struct|MakeVineVisualization (.curlnoisescale (Variables|Default|GetVV)) (Variables|ViewEdit|GetCurlNoiseFre) (.perlinnoisescale (Variables|Default|GetVV)) (Variables|ViewEdit|GetPerlinNoiseFre) 5.0 0.1 0.35 3.0 5.0 (.curvecontrol (Variables|Default|GetVV)))))))

(fn FetchSceneFoliage
  (bind _billboard (Variables|Default|GetBillboard))
  (Transformation|SetActorLocation "0, 0, 0" false false)
  (Transformation|SetWorldLocation _billboard (Transformation|GetWorldLocation _billboard) false false)
  (Utilities|FlowControl|Sequence
    (:then_0
      (Class|VineContainer|ImportFoliagetoTransformArray (Variables|Default|GetTubeVineType)))
    (:then_1
      (Class|VineContainer|ImportFoliagetoTransformArray (Variables|Default|GetPlaneVineType)))
    (:then_2
      (Class|VineContainer|ImportFoliagetoTransformArray (Variables|Default|GetTargetInstances)))))

(fn RevertSceneFoliage
  (Development|SetHiddeninGame (Variables|DynamicMeshActor|GetDynamicMeshComponent) false false)
  (Utilities|FlowControl|Sequence
    (:then_0
      (Class|VineContainer|ExportTransformArraytoFoliage (Variables|Default|GetTubeVineType)))
    (:then_1
      (Class|VineContainer|ExportTransformArraytoFoliage (Variables|Default|GetPlaneVineType)))
    (:then_2
      (Class|VineContainer|ExportTransformArraytoFoliage (Variables|Default|GetTargetInstances)))))

(fn CleanAllMesh
  (Class|VineContainer|Clean))