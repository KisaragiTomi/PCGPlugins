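; Scratch actor in TreeWindData for trying Geometry Script operations on a merged static mesh through a DynamicMeshComponent.
; One custom event rights the actor by applying a shortest-arc quaternion from its up vector to world Z.
; Another copies the mesh asset into the dynamic mesh and welds its edges with a very large tolerance.
; The remaining graph is disconnected experiments: normal and ray-query debugging, spline sweeps, UV edits and copying back to the asset.
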(event `CustomEvent`
  (`self.K2_SetActorRotation` (`KismetMathLibrary.Quat_Rotator` (* (`KismetMathLibrary.Conv_RotatorToQuaternion` (`self.K2_GetActorRotation`)) (`KismetMathLibrary.Quat_FindBetweenNormals` (`self.GetActorUpVector`) (0.0 0.0 1.0))))))

(event `CustomEvent_1`
  (bind _returnvalue (`BaseDynamicMeshComponent.GetDynamicMesh` (`self.DynamicMeshComponent`)))
  (bind _returnvalue_2 (`DynamicMesh.Reset` _returnvalue))
  (`GeometryScriptLibrary_StaticMeshFunctions.CopyMeshFromStaticMeshV2` "/Game/MyProject/_GENERATED/KLW/Merge_9B6BA5D1.Merge_9B6BA5D1" _returnvalue_2 (struct) (struct) true null
    (:`Success`
      (`GeometryScriptLibrary_MeshRepairFunctions.WeldMeshEdges` _returnvalue (make `GeometryScriptWeldEdgesOptions` 111.0 false) null))))

(fn `UserConstructionScript`)